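; BP_Crowd_Female1 is a female crowd character that wanders the navmesh on its own.
; From BeginPlay, MoveRandom picks a random navigable point around the actor's current location and sends it there with AI MoveTo.
; Each successful move calls MoveRandom again, then plays a non-looping walk animation and sets the walk speed.
; The failure path is unhandled, so a failed move ends the loop.
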(event `self.ReceiveBeginPlay`
  (`self.MoveRandom`))

(event `MoveRandom`
  (bind _randomlocation (`NavigationSystemV1.K2_GetRandomLocationInNavigableRadius` (`self.K2_GetActorLocation`) 1000.0 null null))
  (`|AIMoveTo` self _randomlocation null 150.0
    (:`OnSuccess`
      (`self.MoveRandom`)
      (`|ExecutionSequence`
        (:`then_0`
          (`SkeletalMeshComponent.PlayAnimation` (`self.Mesh`) "/Game/LJC/Assets/Sketchfab/Crowd-female/Female_Walk_Anim.Female_Walk_Anim" false)
          (set `CharacterMovementComponent.MaxWalkSpeed` 100.0 (`self.CharacterMovement`)))))))

(fn `UserConstructionScript`)