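; Treasure chest actor that opens when its Interract event fires.
; A DoOnce limits opening to a single time, playing the lid animation unlooped on both the Top and SkeletalMesh components.
; When BP_MainPlayer begins overlapping TriggerLeft, that component is made visible in game; beginning overlap with Box hides it again.
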(event `/Game/LJC/BP/BP_TreasureBox_Interface.Interract`
  (`/Engine/EditorBlueprintResources/StandardMacros.DoOnce` false
    (:`Completed`
      (`SkeletalMeshComponent.PlayAnimation` (`self.Top`) "/Game/LJC/Assets/Sketchfab/treasure-chest/source/treasurechest_Lid_Anim.treasurechest_Lid_Anim" false)
      (`SkeletalMeshComponent.PlayAnimation` (`self.SkeletalMesh`) "/Game/LJC/Assets/Sketchfab/treasure-chest/source/treasurechest_Lid_Anim.treasurechest_Lid_Anim" false))))

(event `self.Trigger Left.OnComponentBeginOverlap`
  (params (OverlappedComponent :type "PrimitiveComponent Object Reference") (OtherActor :type "Actor Object Reference") (OtherComp :type "PrimitiveComponent Object Reference") (OtherBodyIndex :type Integer) (bFromSweep :type Boolean) (SweepResult :type "HitResult Structure (by ref)"))
  (cast `/Game/KJY/BluePrint/BP_MainPlayer` OtherActor)
  (`SceneComponent.SetHiddenInGame` (`self.Trigger Left`) false false))

(event `self.Box.OnComponentBeginOverlap`
  (params (OverlappedComponent :type "PrimitiveComponent Object Reference") (OtherActor :type "Actor Object Reference") (OtherComp :type "PrimitiveComponent Object Reference") (OtherBodyIndex :type Integer) (bFromSweep :type Boolean) (SweepResult :type "HitResult Structure (by ref)"))
  (cast `/Game/KJY/BluePrint/BP_MainPlayer` OtherActor)
  (`SceneComponent.SetHiddenInGame` (`self.Trigger Left`) true false))

(fn `UserConstructionScript`)