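; AI controller Blueprint that sets up Blackboard data for the pawn it possesses.
; On possess it loads the BP_Town Blackboard, stores the pawn's location as HomeLoc, and zeroes IdleLoc and TargetLoc.
; The branch condition is fixed to true, so the RunBehaviorTree call for BP_TownA on the false path never executes.
; A random reachable point lookup around the pawn is present but unused.
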(event `self.ReceivePossess`
  (params (PossessedPawn :type "Pawn Object Reference"))
  (if true
    (`self.UseBlackboard` "/Game/LJC/BP/BP_Town.BP_Town")
    (`BlackboardComponent.SetValueAsVector` (`self.Blackboard`) (`self.HomeLoc`) (`self.K2_GetActorLocation` (`self.K2_GetPawn`)))
    (`BlackboardComponent.SetValueAsFloat` (`self.Blackboard`) (`self.IdleLoc`) 0.0)
    (`BlackboardComponent.SetValueAsVector` (`self.Blackboard`) (`self.TargetLoc`) (0.0 0.0 0.0))
    (else
      (`self.RunBehaviorTree` "/Game/LJC/BP/BP_TownA.BP_TownA"))))

(fn `UserConstructionScript`)