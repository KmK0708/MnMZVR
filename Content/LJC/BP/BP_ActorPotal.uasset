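; BP_ActorPotal is a portal actor that moves the player character to a destination when it touches the portal.
; BeginPlay casts player character 0 to BP_MainPlayer and caches it if not already set.
; The static mesh's begin overlap checks for that player and sets its location to DestinationLocation without sweeping.
; The construction script places an Arrow component using TeleportLocation as its relative transform, a separate variable from the DestinationLocation used on overlap.
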(event `self.ReceiveBeginPlay`
  (`self.MainPlayer`
    (:`then`)
    (:`else`
      (bind _asbp_main_player (cast `/Game/KJY/BluePrint/BP_MainPlayer` (`GameplayStatics.GetPlayerCharacter` 0)))
      (set `self.MainPlayer` _asbp_main_player))))

(event `self.StaticMesh.OnComponentBeginOverlap`
  (params (OverlappedComponent :type "PrimitiveComponent Object Reference") (OtherActor :type "Actor Object Reference") (OtherComp :type "PrimitiveComponent Object Reference") (OtherBodyIndex :type Integer) (bFromSweep :type Boolean) (SweepResult :type "HitResult Structure (by ref)"))
  (bind _mainplayer (`self.MainPlayer`))
  (if (== OtherActor _mainplayer)
    (`self.K2_SetActorLocation` _mainplayer (`self.DestinationLocation`) false false)))

(fn `UserConstructionScript`
  (`SceneComponent.K2_SetRelativeTransform` (`self.Arrow`) (`self.TeleportLocation`) false false))