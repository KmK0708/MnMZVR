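; BP_BrokenSword is a grabbable broken sword item that builds on a parent class.
; On BeginPlay it runs the parent logic, then, if the GrabComponent is valid, passes it the item's SlotType along with sword-specific slotted and holster transforms and a default world scale.
; The transforms shrink the sword when slotted or holstered relative to its in-world size; overlap and tick events are unused.
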(event `self.ReceiveBeginPlay`
  (bind _grabcomponent (`self.GrabComponent`))
  (`parent.ReceiveBeginPlay`)
  (`/Engine/EditorBlueprintResources/StandardMacros.IsValid` _grabcomponent
    (:`Is Valid`
      (set `/Game/VR_Inventorys/Blueprints/BP_VRM_GrabComponent.SlotType` (`self.Slot Type`) _grabcomponent)
      (set `/Game/VR_Inventorys/Blueprints/BP_VRM_GrabComponent.Slotted Transfrom` (`KismetMathLibrary.MakeTransform` (0.0 0.0 -5.0) (struct) (0.15 0.15 0.15)) _grabcomponent)
      (set `/Game/VR_Inventorys/Blueprints/BP_VRM_GrabComponent.Holster Transform` (`KismetMathLibrary.MakeTransform` (0.0 -10.0 0.0) (struct :`Pitch` -90.0 :`Yaw` 90.0) (0.15 0.15 0.15)) _grabcomponent)
      (set `/Game/VR_Inventorys/Blueprints/BP_VRM_GrabComponent.Default World scale` (0.4 0.4 0.4) _grabcomponent) ; Size you want the actor to be when In world
    )))

(fn `UserConstructionScript`
  (`parent.UserConstructionScript`))