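; Weapon shop actor that shows a shop UI and plays voice lines as the player enters and leaves its box.
; BeginPlay fills its weapon inventory from DT_Weaponinfo, using expected-weapon enum names as row names.
; After a short delay, entry spawns BP_WeaponShopUI once or re-shows it, while exit hides it.
; Both toggle the player's right widget-interaction debug display; the sell-box overlap is an empty stub.
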(event `self.ReceiveBeginPlay`
  (bind _weaponinvenexpected (`self.WeaponInvenExpected`))
  ;[1 1 1] 무기 데이터테이블 가져오기
  (bind _asbp_main_player_child (cast `/Game/KJY/BluePrint/BP_MainPlayer_Child` (`GameplayStatics.GetPlayerCharacter` 0)))
  (set `self.PlayerInfo` _asbp_main_player_child)
  (for _index (range (`KismetArrayLibrary.Array_Length` _weaponinvenexpected))
    (bind _returnvalue (`|GetDataTableRow` "/Game/KJY/BluePrint/Items/DT_Weaponinfo.DT_Weaponinfo" (`KismetStringLibrary.Conv_StringToName` (`|GetEnumeratorNameAsString` (`|GetArrayItem` _weaponinvenexpected _index))))
      (:`then`
        (`KismetArrayLibrary.Array_AddUnique` (`self.WeaponInventory`) _returnvalue)))))

(event `self.ShopBoxComp.OnComponentBeginOverlap`
  (params (OverlappedComponent :type "PrimitiveComponent Object Reference") (OtherActor :type "Actor Object Reference") (OtherComp :type "PrimitiveComponent Object Reference") (OtherBodyIndex :type Integer) (bFromSweep :type Boolean) (SweepResult :type "HitResult Structure (by ref)"))
  (bind _returnvalue (`GameplayStatics.GetPlayerCharacter` 0))
  (if (== OtherActor _returnvalue)
    (bind _asbp_main_player_child (cast `/Game/KJY/BluePrint/BP_MainPlayer_Child` _returnvalue))
    (`KismetSystemLibrary.Delay` 0.4)
    (bind _spawnweaponstore (`self.SpawnWeaponStore`)
      (:`then`
        (set `/Game/KJY/BluePrint/Items/Shop/WeaponShop/BP_WeaponShopUI.BPWeaponShop` self _spawnweaponstore)
        (`SceneComponent.SetVisibility` (`/Game/KJY/BluePrint/Items/Shop/WeaponShop/BP_WeaponShopUI.WeaponShopUI` _spawnweaponstore) true false)
        (bind _rightwidgetinter (`/Game/KJY/BluePrint/BP_MainPlayer_Child.RightWidgetInter` _asbp_main_player_child))
        (set `WidgetInteractionComponent.bShowDebug` true _rightwidgetinter)
        (`GameplayStatics.PlaySound2D` "/Game/KJY/SFX/WeaponShop/Elz_greetings_Cue.Elz_greetings_Cue" 1.0 1.0 0.0 null null))
      (:`else`
        (bind _returnvalue_2 (`|SpawnActorFromClass` "/Game/KJY/BluePrint/Items/Shop/WeaponShop/BP_WeaponShopUI.BP_WeaponShopUI_C" (`SceneComponent.K2_GetComponentToWorld` (`self.SpawnUI`)) "Undefined" "OverrideRootScale" null null))
        (set `/Game/KJY/BluePrint/Items/Shop/WeaponShop/BP_WeaponShopUI.BPWeaponShop` self _returnvalue_2)
        (set `self.SpawnWeaponStore` _returnvalue_2)
        (`SceneComponent.K2_SetWorldTransform` (`/Game/KJY/BluePrint/Items/Shop/WeaponShop/BP_WeaponShopUI.WeaponShopSpawnUI` _returnvalue_2) (`SceneComponent.K2_GetComponentToWorld` (`self.SpawnItemLocation`)) false false)
        (set `WidgetInteractionComponent.bShowDebug` true _rightwidgetinter)
        (`GameplayStatics.PlaySound2D` "/Game/KJY/SFX/WeaponShop/Elz_hello_Cue.Elz_hello_Cue" 1.0 1.0 0.0 null null)))))

(event `self.ShopBoxComp.OnComponentEndOverlap`
  (params (OverlappedComponent :type "PrimitiveComponent Object Reference") (OtherActor :type "Actor Object Reference") (OtherComp :type "PrimitiveComponent Object Reference") (OtherBodyIndex :type Integer))
  (bind _returnvalue (`SceneComponent.K2_GetComponentLocation` (`self.SpawnUI`)))
  (if (== OtherActor (`GameplayStatics.GetPlayerCharacter` 0))
    (`KismetSystemLibrary.Delay` 0.5)
    (`SceneComponent.SetVisibility` (`/Game/KJY/BluePrint/Items/Shop/WeaponShop/BP_WeaponShopUI.WeaponShopUI` (`self.SpawnWeaponStore`)) false false)
    (set `WidgetInteractionComponent.bShowDebug` false (`/Game/KJY/BluePrint/BP_MainPlayer_Child.RightWidgetInter` (stale `self.ShopBoxComp.OnComponentBeginOverlap` _asbp_main_player_child)))
    (if (`KismetMathLibrary.Conv_IntToBool` (`KismetMathLibrary.RandomIntegerInRange` 0 1))
      (`GameplayStatics.PlaySoundAtLocation` "/Game/KJY/SFX/WeaponShop/Elz_comeagain_Cue.Elz_comeagain_Cue" _returnvalue (struct) 1.0 1.0 0.0 null null null null)
      (else
        (`GameplayStatics.PlaySoundAtLocation` "/Game/KJY/SFX/WeaponShop/Elz_farewell_Cue.Elz_farewell_Cue" _returnvalue (struct) 1.0 1.0 0.0 null null null null)))))

(event `self.SellBoxComp.OnComponentBeginOverlap`
  (params (OverlappedComponent :type "PrimitiveComponent Object Reference") (OtherActor :type "Actor Object Reference") (OtherComp :type "PrimitiveComponent Object Reference") (OtherBodyIndex :type Integer) (bFromSweep :type Boolean) (SweepResult :type "HitResult Structure (by ref)")))

(fn `UserConstructionScript`)