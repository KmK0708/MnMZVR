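; BP_WeaponShopUI is the actor that hosts the weapon shop widget and builds the shop's weapon inventory.
; On BeginPlay, if the shop is not flagged open, it looks up each expected weapon enum by name in DT_Weaponinfo and adds found rows uniquely to its inventory.
; It then calls CallWeaponShop, which hands the WB_WeaponShop widget references to the level's BP_WeaponShop and to itself.
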(event `self.ReceiveBeginPlay`
  (bind _weaponinvexpected (`self.WeaponInvExpected`))
  (if (not (`self.WeaponShopOpen?`))
    (for _index (range (`KismetArrayLibrary.Array_Length` _weaponinvexpected))
      (bind _returnvalue (`|GetDataTableRow` "/Game/KJY/BluePrint/Items/DT_Weaponinfo.DT_Weaponinfo" (`KismetStringLibrary.Conv_StringToName` (`|GetEnumeratorNameAsString` (`|GetArrayItem` _weaponinvexpected _index))))
        (:`then`
          (`KismetArrayLibrary.Array_AddUnique` (`self.WeaponInventoy`) _returnvalue))))
    (`self.CallWeaponShop`)))

(event `CallWeaponShop`
  (bind _returnvalue (`GameplayStatics.GetActorOfClass` "/Game/KJY/BluePrint/Items/Shop/WeaponShop/BP_WeaponShop.BP_WeaponShop_C"))
  (bind _aswb_weapon_shop (cast `/Game/KJY/BluePrint/Items/Shop/WeaponShop/WB_WeaponShop` (`WidgetComponent.GetWidget` (`self.WeaponShopUI`))))
  (set `/Game/KJY/BluePrint/Items/Shop/WeaponShop/WB_WeaponShop.BPWeaponShopRef` _returnvalue _aswb_weapon_shop)
  (set `/Game/KJY/BluePrint/Items/Shop/WeaponShop/WB_WeaponShop.WeaponShopMenu` self _aswb_weapon_shop))

(fn `UserConstructionScript`)