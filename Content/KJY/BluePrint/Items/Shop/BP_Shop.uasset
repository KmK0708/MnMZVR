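; BP_Shop is a shop actor that shows a store UI near the player and buys dropped items for money.
; BeginPlay fills Inventory from DT_ItemInfo using the InventoryExpected list.
; ShopBoxComp overlaps, after short delays, spawn or toggle a reused BP_StoreUI and the player's widget-interaction debug display.
; SellBox pays, plays a coin sound and destroys BP_DropItemBase actors, pricing by the first Inventory entry's index rather than the dropped item.
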(event `self.ReceiveBeginPlay`
  (bind _inventoryexpected (`self.InventoryExpected`))
  ;[1 1 1] 데이터테이블 가져오기
  (bind _asbp_main_player_child (cast `/Game/KJY/BluePrint/BP_MainPlayer_Child` (`GameplayStatics.GetPlayerCharacter` 0)))
  (set `self.PlayerInfo` _asbp_main_player_child)
  (for _index (range (`KismetArrayLibrary.Array_Length` _inventoryexpected))
    (bind _returnvalue (`|GetDataTableRow` "/Game/KJY/BluePrint/Items/DT_ItemInfo.DT_ItemInfo" (`KismetStringLibrary.Conv_StringToName` (`|GetEnumeratorNameAsString` (`|GetArrayItem` _inventoryexpected _index))))
      (:`then`
        (`KismetArrayLibrary.Array_AddUnique` (`self.Inventory`) _returnvalue)))))

(event `self.ShopBoxComp.OnComponentBeginOverlap`
  (params (OverlappedComponent :type "PrimitiveComponent Object Reference") (OtherActor :type "Actor Object Reference") (OtherComp :type "PrimitiveComponent Object Reference") (OtherBodyIndex :type Integer) (bFromSweep :type Boolean) (SweepResult :type "HitResult Structure (by ref)"))
  (bind _returnvalue (`GameplayStatics.GetPlayerCharacter` 0))
  (if (== OtherActor _returnvalue)
    (bind _asbp_main_player_child (cast `/Game/KJY/BluePrint/BP_MainPlayer_Child` _returnvalue))
    (`KismetSystemLibrary.Delay` 0.4)
    (bind _spawnstore (`self.SpawnStore`)
      (:`then`
        (set `/Game/KJY/BluePrint/Items/Shop/BP_StoreUI.BPShopRef` self _spawnstore)
        (`SceneComponent.SetVisibility` (`/Game/KJY/BluePrint/Items/Shop/BP_StoreUI.ShopUI` _spawnstore) true false)
        (bind _rightwidgetinter (`/Game/KJY/BluePrint/BP_MainPlayer_Child.RightWidgetInter` _asbp_main_player_child))
        (set `WidgetInteractionComponent.bShowDebug` true _rightwidgetinter))
      (:`else`
        (bind _returnvalue_2 (`|SpawnActorFromClass` "/Game/KJY/BluePrint/Items/Shop/BP_StoreUI.BP_StoreUI_C" (`SceneComponent.K2_GetComponentToWorld` (`self.Scene`)) "Undefined" "OverrideRootScale" null null))
        (set `/Game/KJY/BluePrint/Items/Shop/BP_StoreUI.BPShopRef` self _returnvalue_2)
        (set `self.SpawnStore` _returnvalue_2)
        (`SceneComponent.K2_SetWorldTransform` (`/Game/KJY/BluePrint/Items/Shop/BP_StoreUI.SpawnPosRef` _returnvalue_2) (`SceneComponent.K2_GetComponentToWorld` (`self.SpawnLocation`)) false false)
        (set `WidgetInteractionComponent.bShowDebug` true _rightwidgetinter)))))

(event `self.ShopBoxComp.OnComponentEndOverlap`
  (params (OverlappedComponent :type "PrimitiveComponent Object Reference") (OtherActor :type "Actor Object Reference") (OtherComp :type "PrimitiveComponent Object Reference") (OtherBodyIndex :type Integer))
  (if (== OtherActor (`GameplayStatics.GetPlayerCharacter` 0))
    (`KismetSystemLibrary.Delay` 0.5)
    (`SceneComponent.SetVisibility` (`/Game/KJY/BluePrint/Items/Shop/BP_StoreUI.ShopUI` (`self.SpawnStore`)) false false)
    (set `WidgetInteractionComponent.bShowDebug` false (`/Game/KJY/BluePrint/BP_MainPlayer_Child.RightWidgetInter` (stale `self.ShopBoxComp.OnComponentBeginOverlap` _asbp_main_player_child)))))

(event `self.SellBox.OnComponentBeginOverlap`
  (params (OverlappedComponent :type "PrimitiveComponent Object Reference") (OtherActor :type "Actor Object Reference") (OtherComp :type "PrimitiveComponent Object Reference") (OtherBodyIndex :type Integer) (bFromSweep :type Boolean) (SweepResult :type "HitResult Structure (by ref)"))
  (bind _playerinfo (`self.PlayerInfo`))
  (bind _playerinfo_2 (`self.PlayerInfo`))
  (bind _playerinfo_3 (`self.PlayerInfo`))
  (bind _playerinfo_4 (`self.PlayerInfo`))
  (bind _playerinfo_5 (`self.PlayerInfo`))
  (bind (_itemclass _itemname _itemimage _currentstack _maxstack _itemindex) (break `/Game/KJY/BluePrint/Items/ItemStruct` (`|GetArrayItem` (`self.Inventory`))))
  (bind _asbp_drop_item_base (cast `/Game/KJY/BluePrint/Items/BP_DropItemBase` OtherActor))
  (if true
    (if (== _itemindex 1)
      (`KismetSystemLibrary.PrintString` "healthpotion")
      (set `MainPlayer.PlayerMoney` (+ (`MainPlayer.PlayerMoney` _playerinfo_2) 25) _playerinfo_2)
      (`GameplayStatics.PlaySound2D` "/Game/MedFntSFX/wavs/Environment/coins_pickup_shake_01.coins_pickup_shake_01" 1.0 1.0 0.0 null null)
      (`self.K2_DestroyActor` _asbp_drop_item_base)
      (elif (== _itemindex 2)
        (`KismetSystemLibrary.PrintString` "strange")
        (set `MainPlayer.PlayerMoney` (+ (`MainPlayer.PlayerMoney` _playerinfo_3) 10) _playerinfo_3)
        (`GameplayStatics.PlaySound2D` "/Game/MedFntSFX/wavs/Environment/coins_pickup_shake_02.coins_pickup_shake_02" 1.0 1.0 0.0 null null)
        (`self.K2_DestroyActor` _asbp_drop_item_base)
        (elif (== _itemindex 4)
          (`KismetSystemLibrary.PrintString` "broken")
          (set `MainPlayer.PlayerMoney` (+ (`MainPlayer.PlayerMoney` _playerinfo_4) 100) _playerinfo_4)
          (`GameplayStatics.PlaySound2D` "/Game/MedFntSFX/wavs/Environment/coins_pickup_shake_03.coins_pickup_shake_03" 1.0 1.0 0.0 null null)
          (`self.K2_DestroyActor` _asbp_drop_item_base)
          (elif (== _itemindex 5)
            (`KismetSystemLibrary.PrintString` "wood")
            (set `MainPlayer.PlayerMoney` (+ (`MainPlayer.PlayerMoney` _playerinfo_5) 5) _playerinfo_5)
            (`GameplayStatics.PlaySound2D` "/Game/MedFntSFX/wavs/Environment/coins_pickup_shake_05.coins_pickup_shake_05" 1.0 1.0 0.0 null null)
            (`self.K2_DestroyActor` _asbp_drop_item_base)
            (elif (== _itemindex 6)
              (`KismetSystemLibrary.PrintString` "scroll")
              (set `MainPlayer.PlayerMoney` (+ (`MainPlayer.PlayerMoney` _playerinfo) 75) _playerinfo)
              (`GameplayStatics.PlaySound2D` "/Game/MedFntSFX/wavs/Environment/coins_pickup_shake_05.coins_pickup_shake_05" 1.0 1.0 0.0 null null)
              (`self.K2_DestroyActor` _asbp_drop_item_base)
              (else
                (`KismetSystemLibrary.PrintString` "none" true true (struct :`R` 1.0 :`G` 0.974041 :`B` 0.953415 :`A` 1.0))))))))))

(fn `UserConstructionScript`)