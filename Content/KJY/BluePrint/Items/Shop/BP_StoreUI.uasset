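; BP_StoreUI is an actor that hosts the shop's widget and supplies the list of items it stocks.
; On BeginPlay, if the shop is not open, it resolves each InventoryExpected enum name as a DT_ItemInfo row and adds found rows uniquely to Inventory.
; CallShowShop then gets the WB_Shop from the ShopUI widget component and hands it references to the level's BP_Shop and to itself.
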(event `self.ReceiveBeginPlay`
  (bind _inventoryexpected (`self.InventoryExpected`))
  (if (not (`self.ShopOpen?`))
    (for _index (range (`KismetArrayLibrary.Array_Length` _inventoryexpected))
      (bind _returnvalue (`|GetDataTableRow` "/Game/KJY/BluePrint/Items/DT_ItemInfo.DT_ItemInfo" (`KismetStringLibrary.Conv_StringToName` (`|GetEnumeratorNameAsString` (`|GetArrayItem` _inventoryexpected _index))))
        (:`then`
          (`KismetArrayLibrary.Array_AddUnique` (`self.Inventory`) _returnvalue))))
    (`self.CallShowShop`)))

(event `CallShowShop`
  (bind _returnvalue (`GameplayStatics.GetActorOfClass` "/Game/KJY/BluePrint/Items/Shop/BP_Shop.BP_Shop_C"))
  (bind _aswb_shop (cast `/Game/KJY/BluePrint/Items/Shop/WB_Shop` (`WidgetComponent.GetWidget` (`self.ShopUI`))))
  (set `/Game/KJY/BluePrint/Items/Shop/WB_Shop.BPShopRef` _returnvalue _aswb_shop)
  (set `/Game/KJY/BluePrint/Items/Shop/WB_Shop.ShopMenu` self _aswb_shop))

(fn `UserConstructionScript`)