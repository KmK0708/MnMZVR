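; Base actor for dropped items that the player can pick up into their inventory or grab and slot.
; The construction script fills the item info from DT_ItemInfo, using the ItemName enum's string as the row name.
; BeginPlay configures the grab component's slot type, slotted and holster transforms, and world scale.
; Interact, when allowed, passes the item info to BP_MainPlayer's PickupItem and optionally destroys the actor.
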(event `self.ReceiveBeginPlay`
  (bind _grabcomponent (`self.GrabComponent`))
  (`/Engine/EditorBlueprintResources/StandardMacros.IsValid` _grabcomponent
    (:`Is Valid`
      (set `/Game/VR_Inventorys/Blueprints/BP_VRM_GrabComponent.SlotType` (`self.Slot Type`) _grabcomponent)
      (set `/Game/VR_Inventorys/Blueprints/BP_VRM_GrabComponent.Slotted Transfrom` (`KismetMathLibrary.MakeTransform` (0.0 0.0 -5.0) (struct) (0.5 0.5 0.5)) _grabcomponent)
      (set `/Game/VR_Inventorys/Blueprints/BP_VRM_GrabComponent.Holster Transform` (`KismetMathLibrary.MakeTransform` (0.0 -10.0 0.0) (struct :`Pitch` -90.0 :`Yaw` 90.0)) _grabcomponent)
      (set `/Game/VR_Inventorys/Blueprints/BP_VRM_GrabComponent.Default World scale` (1.0 1.0 1.0) _grabcomponent) ; Size you want the actor to be when In world
    )))

(event `/Game/KJY/BluePrint/Interface/BPI_Interact.Interact`
  (if (`self.Interactable?`)
    (bind _asbp_main_player (cast `/Game/KJY/BluePrint/BP_MainPlayer` (`GameplayStatics.GetPlayerCharacter` 0)))
    (`/Game/KJY/BluePrint/BP_MainPlayer.Pickup Item` _asbp_main_player (`self.Iteminfo`))
    (if (`self.Destroy?`)
      (`self.K2_DestroyActor`))))

(fn `UserConstructionScript`
  (bind _returnvalue (`|GetDataTableRow` "/Game/KJY/BluePrint/Items/DT_ItemInfo.DT_ItemInfo" (`KismetStringLibrary.Conv_StringToName` (`|GetEnumeratorNameAsString` (`self.ItemName`))))
    (:`then`
      (set `self.Iteminfo` _returnvalue))))