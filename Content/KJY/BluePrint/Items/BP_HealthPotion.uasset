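; Health potion item Blueprint that sets itself up as a grabbable, slottable pickup.
; On BeginPlay it calls the parent, then configures a valid GrabComponent with its slot type, slotted and holster transforms, and default world scale.
; The potion shrinks to half size when slotted and is full size when holstered or in the world.
; Interact is an empty stub, so no healing logic lives in this graph.
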(event `self.ReceiveBeginPlay`
  (bind _grabcomponent_0 (`self.GrabComponent_0`))
  (`parent.ReceiveBeginPlay`)
  (`/Engine/EditorBlueprintResources/StandardMacros.IsValid` _grabcomponent_0
    (:`Is Valid`
      (set `/Game/VR_Inventorys/Blueprints/BP_VRM_GrabComponent.SlotType` (`self.Slot Type_0`) _grabcomponent_0)
      (set `/Game/VR_Inventorys/Blueprints/BP_VRM_GrabComponent.Slotted Transfrom` (`KismetMathLibrary.MakeTransform` (0.0 0.0 -3.5) (struct :`Yaw` 90.0) (0.5 0.5 0.5)) _grabcomponent_0)
      (set `/Game/VR_Inventorys/Blueprints/BP_VRM_GrabComponent.Holster Transform` (`KismetMathLibrary.MakeTransform` (0.0 0.0 0.0) (struct :`Roll` -90.0)) _grabcomponent_0)
      (set `/Game/VR_Inventorys/Blueprints/BP_VRM_GrabComponent.Default World scale` (1.0 1.0 1.0) _grabcomponent_0) ; Size you want the actor to be when In world
    )))

(event `/Game/KJY/BluePrint/Interface/BPI_Interact.Interact`)

(fn `UserConstructionScript`
  (`parent.UserConstructionScript`))