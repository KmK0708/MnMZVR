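; BP_SoulStone is a grabbable soul stone item that can be slotted or holstered.
; On BeginPlay it configures its GrabComponent with the slot type, slotted and holster transforms, and a default world scale, giving the stone a different size in each state.
; The sphere overlap event is empty, so any other behavior comes from its parent class or components.
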(event `self.ReceiveBeginPlay`
  (bind _grabcomponent (`self.GrabComponent`))
  (`parent.ReceiveBeginPlay`)
  (`/Engine/EditorBlueprintResources/StandardMacros.IsValid` _grabcomponent
    (:`Is Valid`
      (set `/Game/VR_Inventorys/Blueprints/BP_VRM_GrabComponent.SlotType` (`self.Slot Type`) _grabcomponent)
      (set `/Game/VR_Inventorys/Blueprints/BP_VRM_GrabComponent.Slotted Transfrom` (`KismetMathLibrary.MakeTransform` (0.0 0.0 -5.0) (struct) (0.25 0.25 0.25)) _grabcomponent)
      (set `/Game/VR_Inventorys/Blueprints/BP_VRM_GrabComponent.Holster Transform` (`KismetMathLibrary.MakeTransform` (0.0 -10.0 0.0) (struct :`Pitch` -90.0 :`Yaw` 90.0) (0.5 0.5 0.5)) _grabcomponent)
      (set `/Game/VR_Inventorys/Blueprints/BP_VRM_GrabComponent.Default World scale` (0.5 0.5 0.5) _grabcomponent) ; Size you want the actor to be when In world
    )))

(event `self.SphereComp.OnComponentBeginOverlap`
  (params (OverlappedComponent :type "PrimitiveComponent Object Reference") (OtherActor :type "Actor Object Reference") (OtherComp :type "PrimitiveComponent Object Reference") (OtherBodyIndex :type Integer) (bFromSweep :type Boolean) (SweepResult :type "HitResult Structure (by ref)")))

(fn `UserConstructionScript`
  (`parent.UserConstructionScript`))