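; BP_InventoryComp is an overlap-driven inventory slot component that snaps a BP_InventoryCube onto itself once a motion controller releases it.
; On begin overlap, an empty slot stores a cube held by any controller other than ControllerToIgnore, and end overlap clears it.
; Tick polls the stored cube and, while it has no MotionController, attaches it to the component with snapped location and rotation, keeping world scale.
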(event `self.ReceiveBeginPlay`
  (add `self.OnComponentBeginOverlap` (delegate `Begin Overlap`))
  (add `self.OnComponentEndOverlap` (delegate `End Overlap`)))

(event `Begin Overlap` :!signature `self.OnComponentBeginOverlap`
  (params (OverlappedComponent :type "PrimitiveComponent Object Reference") (OtherActor :type "Actor Object Reference") (OtherComp :type "PrimitiveComponent Object Reference") (OtherBodyIndex :type Integer) (bFromSweep :type Boolean) (SweepResult :type "HitResult Structure (by ref)"))
  (bind _controllertoignore (`self.ControllerToIgnore`))
  (`/Engine/EditorBlueprintResources/StandardMacros.IsValid` (`self.GrabActor`)
    (:`Is Not Valid`
      (bind _asbp_inventory_cube (cast `/Game/KJY/BluePrint/BP_InventoryCube` OtherActor))
      (bind _motion_controller (`/Game/KJY/BluePrint/BP_InventoryCube.Motion Controller` _asbp_inventory_cube))
      (`/Engine/EditorBlueprintResources/StandardMacros.IsValid` _motion_controller
        (:`Is Valid`
          (`/Engine/EditorBlueprintResources/StandardMacros.IsValid` _controllertoignore
            (:`Is Valid`
              (if (!= _controllertoignore _motion_controller)
                (set `self.GrabActor` _asbp_inventory_cube :!label _label)))
            (:`Is Not Valid`
              (goto _label))))))))

(event `End Overlap`
  (params (OverlappedComponent :type "PrimitiveComponent Object Reference") (OtherActor :type "Actor Object Reference") (OtherComp :type "PrimitiveComponent Object Reference") (OtherBodyIndex :type Integer))
  (if (== OtherActor (`self.GrabActor`))
    (set `self.GrabActor` null)))

(event `self.ReceiveTick`
  (params (DeltaSeconds :type "Float (single-precision)"))
  (bind _grabactor (`self.GrabActor`))
  (`/Engine/EditorBlueprintResources/StandardMacros.IsValid` _grabactor
    (:`Is Valid`
      (`/Engine/EditorBlueprintResources/StandardMacros.IsValid` (`/Game/KJY/BluePrint/BP_InventoryCube.Motion Controller` _grabactor)
        (:`Is Not Valid`
          (`Actor.K2_AttachToComponent` _grabactor self "None" "SnapToTarget" "SnapToTarget" "KeepWorld" true))))))