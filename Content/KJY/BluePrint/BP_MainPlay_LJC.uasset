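; BP_MainPlay_LJC is a player Blueprint with hand meshes that lets grasp inputs click UI through widget interaction components.
; Enhanced Input grasp actions press and release a simulated left mouse button on each hand's component, with debug prints.
; The left hand presses on Started or Triggered and releases on Completed or Canceled; the right uses only Triggered and Canceled.
; A right-hand forward line trace is left unconnected.
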(event `EnhancedInput|/Game/VRTemplate/Input/Actions/Hands/IA_Hand_Grasp_Left`
  (params (ActionValue :type "Float (double-precision)") (ElapsedSeconds :type "Float (double-precision)") (TriggeredSeconds :type "Float (double-precision)") (InputAction :type "InputAction Object Reference" :default "/Game/VRTemplate/Input/Actions/Hands/IA_Hand_Grasp_Left.IA_Hand_Grasp_Left"))
  (bind _widgetinteraction_0 (`self.WidgetInteraction_0`))
  (:`Triggered`
    (`WidgetInteractionComponent.PressPointerKey` _widgetinteraction_0 "LeftMouseButton" :!label _label))
  (:`Started`
    (goto _label))
  (:`Canceled`
    (`KismetSystemLibrary.PrintString` "2" :!label _label_2)
    (`WidgetInteractionComponent.ReleasePointerKey` _widgetinteraction_0 "LeftMouseButton"))
  (:`Completed`
    (goto _label_2)))

(event `EnhancedInput|/Game/VRTemplate/Input/Actions/Hands/IA_Hand_Grasp_Right`
  (params (ActionValue :type "Float (double-precision)") (ElapsedSeconds :type "Float (double-precision)") (TriggeredSeconds :type "Float (double-precision)") (InputAction :type "InputAction Object Reference" :default "/Game/VRTemplate/Input/Actions/Hands/IA_Hand_Grasp_Right.IA_Hand_Grasp_Right"))
  (bind _uiinteractright (`self.UIInteractRight`))
  (:`Triggered`
    (`KismetSystemLibrary.PrintString` "Hello")
    (`WidgetInteractionComponent.PressPointerKey` _uiinteractright "LeftMouseButton"))
  (:`Canceled`
    (`KismetSystemLibrary.PrintString` "1")
    (`WidgetInteractionComponent.ReleasePointerKey` _uiinteractright "LeftMouseButton")))

(fn `UserConstructionScript`
  (`parent.UserConstructionScript`))