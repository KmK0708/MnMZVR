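; BP_HLA_Inventory is a VR inventory menu actor that shows and hides arrow planes and child inventory slots.
; Appear and OnDisappear play one timeline forward or backward to scale and fade the arrows through a shared dynamic material, hiding the actor after reversing.
; Both events also notify every child BP_Inventory_Slot_BASE.
; Unless PromoExample is set, Tick turns the menu toward the cached BP_VRPawn camera with clamped pitch.
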(event `self.ReceiveBeginPlay`
  ;[1 1 1] start
  (bind _returnvalue (`PrimitiveComponent.CreateDynamicMaterialInstance` (`self.Arrow Plane`) 0 null "None"))
  (set `self.Arrow Dynamic MAT` _returnvalue)
  (`PrimitiveComponent.SetMaterial` (`self.Arrow Plane3`) 0 (`self.Arrow Dynamic MAT`))
  (`PrimitiveComponent.SetMaterial` (`self.Arrow Plane1`) 0 (`self.Arrow Dynamic MAT`))
  (`PrimitiveComponent.SetMaterial` (`self.Arrow Plane2`) 0 (`self.Arrow Dynamic MAT`))
  (`PrimitiveComponent.SetMaterial` (`self.Arrow Plane`) 0 (`self.Arrow Dynamic MAT`)))

(event `Appear`
  ;[1 1 1] Scale and Opacity Transition  for Arrorws
  (`self.SetActorHiddenInGame` false)
  (`|ExecutionSequence`
    (:`then_0`
      (bind (_direction _lerp) (`Timeline|Timeline_0` :!via `PlayFromStart` :!label _label)
        (:`Update`
          (`SceneComponent.SetRelativeScale3D` (`self.Arrows _Pivot`) (`KismetMathLibrary.VLerp` (0.5 0.5 0.5) (1.0 1.0 1.0) _lerp))
          (`MaterialInstanceDynamic.SetScalarParameterValue` (`self.Arrow Dynamic MAT`) "MaxOpacity" (`KismetMathLibrary.Lerp` 0.0 0.75 _lerp)))
        (:`Finished`
          (switch `ETimelineDirection` _direction
            (:`Backward`
              (`self.SetActorHiddenInGame` true))))))
    (:`then_1`
      ;[1 1 1] Appear Slots
      (for _array_element (`self.GetAllChildActors` true)
        (bind _asbp_inventory_slot_base (cast `/Game/VR_Inventorys/Slots/BASE_SLOT/BP_Inventory_Slot_BASE` _array_element))
        (`/Game/VR_Inventorys/Slots/BASE_SLOT/BP_Inventory_Slot_BASE.Appear` _asbp_inventory_slot_base)))))

(event `OnDisappear`
  (`|ExecutionSequence`
    (:`then_0`
      (goto _label :!via `ReverseFromEnd`))
    (:`then_1`
      ;[1 1 1] Dissappear Slots
      (for _array_element (`self.GetAllChildActors` true)
        (bind _asbp_inventory_slot_base (cast `/Game/VR_Inventorys/Slots/BASE_SLOT/BP_Inventory_Slot_BASE` _array_element))
        (`/Game/VR_Inventorys/Slots/BASE_SLOT/BP_Inventory_Slot_BASE.Disappear` _asbp_inventory_slot_base)))))

(event `self.ReceiveTick`
  (params (DeltaSeconds :type "Float (single-precision)"))
  (bind (_returnvalue_roll _returnvalue_pitch _returnvalue_yaw) (`KismetMathLibrary.BreakRotator` (`KismetMathLibrary.FindLookAtRotation` (`SceneComponent.K2_GetComponentLocation` (`self.VR Player Camera`)) (`self.K2_GetActorLocation`))))
  (if (not (`self.Promo Example?`))
    ;[1 1 1] Keep Inventory FACING Player
    (`self.VR Player Camera` ; Happens ONLY once
      (:`then`
        (bind _result (`/Engine/EditorBlueprintResources/StandardMacros.NegateFloat` _returnvalue_pitch)
          (:`  `
            (`self.K2_SetActorRotation` (`KismetMathLibrary.MakeRotator` 0.0 (`KismetMathLibrary.ClampAngle` _result -20.0 20.0) (+ _returnvalue_yaw 180.0))))))
      (:`else`
        ;[1 1 1] Search for Players Vr Camera
        (bind _returnvalue (`GameplayStatics.GetActorOfClass` "/Game/VR_Inventorys/VRTemplate/Blueprints/BP_VRPawn.BP_VRPawn_C"))
        (`/Engine/EditorBlueprintResources/StandardMacros.IsValid` _returnvalue
          (:`Is Valid`
            (set `self.VR Player Camera` (`/Game/VR_Inventorys/VRTemplate/Blueprints/BP_VRPawn.Camera` _returnvalue))))))))

(fn `UserConstructionScript`)