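; BP_Radial_Ring_Inventory is a radial inventory menu for VR that animates itself and its slots in and out.
; Appear unhides the actor, plays a timeline that scales up the plane and fades in its dynamic material, then shows child BP_Inventory_Slot_BASE actors.
; OnDisappear reverses the timeline while hiding the slots, then hides the actor once it finishes.
; An optional PromoExample flag alternates both transitions on Tick for showcase testing.
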(event `self.ReceiveTick`
  (params (DeltaSeconds :type "Float (single-precision)"))
  ;[1 0.5588 0] This Is just for Testing the Appear & disappear Transition & for use as a promo example in the showcase level. Feel free to delete everything in the box Including the Promo example ? Varible If you want, Or just untick Promo Example? when used on a VR player
  (if (`self.Promo Example?`)
    (`KismetSystemLibrary.Delay` 2.0)
    (`/Engine/EditorBlueprintResources/StandardMacros.FlipFlop`
      (:`A`
        (`self.Appear`))
      (:`B`
        (`self.OnDisappear`)))))

(event `self.ReceiveBeginPlay`
  ;[1 1 1] start
  (bind _returnvalue (`PrimitiveComponent.CreateDynamicMaterialInstance` (`self.Plane`) 0 null "None"))
  (bind _output_get (set `self.Plane Material` _returnvalue))
  (`PrimitiveComponent.SetMaterial` (`self.Plane`) 0 _output_get))

(event `Appear`
  ;[1 1 1] Scale and Opacity Transition  for Arrorws
  (`self.SetActorHiddenInGame` false)
  (bind (_direction _lerp) (`Timeline|Timeline_0` :!via `PlayFromStart` :!label _label)
    (:`Update`
      (`SceneComponent.SetRelativeScale3D` (`self.Plane`) (`KismetMathLibrary.VLerp` (0.5 0.5 0.5) (1.0 1.0 1.0) _lerp))
      (`MaterialInstanceDynamic.SetScalarParameterValue` (`self.Plane Material`) "MaxOpacity" (`KismetMathLibrary.Lerp` 0.0 0.75 _lerp)))
    (:`Finished`
      (switch `ETimelineDirection` _direction
        (:`Forward`
          ;[1 1 1] Appear Slots
          (for _array_element (`self.GetAllChildActors` true)
            (bind _asbp_inventory_slot_base (cast `/Game/VR_Inventorys/Slots/BASE_SLOT/BP_Inventory_Slot_BASE` _array_element))
            (`/Game/VR_Inventorys/Slots/BASE_SLOT/BP_Inventory_Slot_BASE.Appear` _asbp_inventory_slot_base)))
        (:`Backward`
          (`self.SetActorHiddenInGame` true))))))

(event `OnDisappear`
  (`|ExecutionSequence`
    (:`then_0`
      (goto _label :!via `ReverseFromEnd`))
    (:`then_1`
      ;[1 1 1] Dissappear Slots
      (for _array_element (`self.GetAllChildActors` true)
        (bind _asbp_inventory_slot_base (cast `/Game/VR_Inventorys/Slots/BASE_SLOT/BP_Inventory_Slot_BASE` _array_element))
        (`/Game/VR_Inventorys/Slots/BASE_SLOT/BP_Inventory_Slot_BASE.Disappear` _asbp_inventory_slot_base)))))

(fn `UserConstructionScript`)