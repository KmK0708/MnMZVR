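; BP_Bag is a VR backpack inventory actor that a hand can grab and release.
; Grabbing hides the player's hand for a pre-authored one, snaps the bag's GrabPoint to the motion controller, then attaches the physics-simulated mesh through a constraint with left-hand haptics.
; Releasing breaks the constraint, restores the hand and, as a temporary solution, parks the bag below the world without physics.
; Construction applies WEIGHT as mass and label text.
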(event `Grab Backpack Inventory`
  (params (`Track Hand` :type "BoxComponent Object Reference") (`Hand Mesh` :type "SkeletalMeshComponent Object Reference") (MotionController :type "MotionControllerComponent Object Reference"))
  (bind (_returnvalue_location _returnvalue_rotation) (`KismetMathLibrary.BreakTransform` (`KismetMathLibrary.ComposeTransforms` (`KismetMathLibrary.InvertTransform` (`SceneComponent.GetRelativeTransform` (`self.grab Point`))) (`SceneComponent.K2_GetComponentToWorld` MotionController))))
  (bind (_returnvalue_location_2 _returnvalue_rotation_2) (`KismetMathLibrary.BreakTransform` (`KismetMathLibrary.TLerp` (`self.GetTransform`) (`KismetMathLibrary.MakeTransform` _returnvalue_location _returnvalue_rotation) 1.0)))
  ;[1 1 1] Grab Backpack
  (`|ExecutionSequence`
    (:`then_0`
      (`/Engine/EditorBlueprintResources/StandardMacros.IsValid` `Hand Mesh`
        (:`Is Valid`
          (`SceneComponent.SetHiddenInGame` `Hand Mesh` true false)
          (set `self.Track Hand` `Track Hand`)
          ;;[1 1 1] Re-Enable Physics if  Inventory Bag was re-Grabbed
          (`PrimitiveComponent.SetSimulatePhysics` (`self.StaticMeshComponent`) true)
          (`PrimitiveComponent.SetCollisionResponseToChannel` (`self.StaticMeshComponent`) "ECC_Pawn" "ECR_Ignore")
          (`self.K2_SetActorTransform` (`KismetMathLibrary.MakeTransform` _returnvalue_location_2 _returnvalue_rotation_2) false true)
          (`PhysicsConstraintComponent.SetConstrainedComponents` (`self.Primary Grab Constraint`) (`self.Track Hand`) "None" (`self.StaticMeshComponent`) "None")
          (`PlayerController.PlayHapticEffect` (`GameplayStatics.GetPlayerController` 0) null "Left" 1.0 false))))
    (:`then_1`
      (`SceneComponent.SetHiddenInGame` (`self.Pre Autherd Hand mesh`) false false))))

(event `Release BackPack`
  ;[1 1 1] Release BackPack
  (`|ExecutionSequence`
    (:`then_0`
      (`/Engine/EditorBlueprintResources/StandardMacros.IsValid` (stale `Grab Backpack Inventory` `Hand Mesh`)
        (:`Is Valid`
          (`SceneComponent.SetHiddenInGame` (stale `Grab Backpack Inventory` `Hand Mesh`) false false)
          (`PhysicsConstraintComponent.BreakConstraint` (`self.Primary Grab Constraint`))
          ;;[1 1 1] Teleport Inventory Bag to a Location (Temp Solution, Until i Find A Better One)
          (`self.K2_SetActorLocation` (0.0 0.0 -1000.0) false true)
          (`PrimitiveComponent.SetSimulatePhysics` (`self.StaticMeshComponent`) false))))
    (:`then_1`
      (`SceneComponent.SetHiddenInGame` (`self.Pre Autherd Hand mesh`) true false))))

(fn `UserConstructionScript`
  (bind _weight (`self.WEIGHT`))
  ;[1 1 1] Set Weight of object at runtime
  (`PrimitiveComponent.SetMassOverrideInKg` (`self.StaticMeshComponent`) "None" _weight true)
  (`TextRenderComponent.K2_SetText` (`self.Weight Info`) (`KismetTextLibrary.Conv_DoubleToText` _weight "HalfToEven")))