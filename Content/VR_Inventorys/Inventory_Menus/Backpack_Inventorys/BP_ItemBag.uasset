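; BP_ItemBag is a physics-driven VR backpack inventory bag that a hand can grab and release.
; Grabbing swaps the hand mesh for a pre-authored one, teleports the bag so GrabPoint aligns with the motion controller, constrains it to the tracked hand and plays left-hand haptics.
; Releasing restores the hand, breaks the constraint, disables physics and parks the bag below the world origin as a stated temporary solution.
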(event `self.ReceiveBeginPlay`)

(event `Grab Backpack Inventory Custom`
  (params (`Track Hand` :type "SphereComponent Object Reference") (`Hand Mesh` :type "SkeletalMeshComponent Object Reference") (MotionController :type "MotionControllerComponent Object Reference"))
  (bind (_returnvalue_location _returnvalue_rotation) (`KismetMathLibrary.BreakTransform` (`KismetMathLibrary.ComposeTransforms` (`KismetMathLibrary.InvertTransform` (`SceneComponent.GetRelativeTransform` (`self.grab Point`))) (`SceneComponent.K2_GetComponentToWorld` MotionController))))
  (bind (_returnvalue_location_2 _returnvalue_rotation_2) (`KismetMathLibrary.BreakTransform` (`KismetMathLibrary.TLerp` (`self.GetTransform`) (`KismetMathLibrary.MakeTransform` _returnvalue_location _returnvalue_rotation) 1.0)))
  ;[1 1 1] Grab Backpack
  (`|ExecutionSequence`
    (:`then_0`
      (`/Engine/EditorBlueprintResources/StandardMacros.IsValid` `Hand Mesh`
        (:`Is Valid`
          (`SceneComponent.SetHiddenInGame` `Hand Mesh` true false)
          (set `self.Track Hand1` `Track Hand`)
          ;;[1 1 1] Re-Enable Physics if  Inventory Bag was re-Grabbed
          (`PrimitiveComponent.SetSimulatePhysics` (`self.StaticMeshComponent`) true)
          (`PrimitiveComponent.SetCollisionResponseToChannel` (`self.StaticMeshComponent`) "ECC_GameTraceChannel11" "ECR_Ignore")
          (`self.K2_SetActorTransform` (`KismetMathLibrary.MakeTransform` _returnvalue_location_2 _returnvalue_rotation_2) false true)
          (`PhysicsConstraintComponent.SetConstrainedComponents` (`self.Primary Grab Constraint`) (`self.Track Hand1`) "None" (`self.StaticMeshComponent`) "None")
          (`PlayerController.PlayHapticEffect` (`GameplayStatics.GetPlayerController` 0) "/Game/VRTemplate/Haptics/GrabHapticEffect.GrabHapticEffect" "Left" 1.0 false))))
    (:`then_1`
      (`SceneComponent.SetHiddenInGame` (`self.Pre Autherd Hand mesh`) false false))))

(event `Release Bag`
  ;[1 1 1] Release BackPack
  (`|ExecutionSequence`
    (:`then_0`
      (`/Engine/EditorBlueprintResources/StandardMacros.IsValid` (stale `Grab Backpack Inventory Custom` `Hand Mesh`)
        (:`Is Valid`
          (`SceneComponent.SetHiddenInGame` (stale `Grab Backpack Inventory Custom` `Hand Mesh`) false false)
          (`PhysicsConstraintComponent.BreakConstraint` (`self.Primary Grab Constraint`))
          ;;[1 1 1] Teleport Inventory Bag to a Location (Temp Solution, Until i Find A Better One)
          (`self.K2_SetActorLocation` (0.0 0.0 -1000.0) false true)
          (`PrimitiveComponent.SetSimulatePhysics` (`self.StaticMeshComponent`) false))))
    (:`then_1`
      (`SceneComponent.SetHiddenInGame` (`self.Pre Autherd Hand mesh`) true false))))

(fn `UserConstructionScript`
  (`parent.UserConstructionScript`))