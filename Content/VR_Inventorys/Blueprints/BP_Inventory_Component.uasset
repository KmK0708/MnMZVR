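; VR inventory manager component that opens and hides six inventory styles: Half-Life Alyx, Dead Space, Deus Ex and three radial rings.
; CallInventory switches on the selected style, placing it beside the hand, before the camera or at a given scene component.
; Each inventory actor spawns on first use, then is cached, teleported and reopened.
; HideInventory closes all valid instances and parks them below the world origin, radials after a delay.
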(event `Hide Inventory`
  (bind _half_life_alyx_style_inventory (`self.Half Life Alyx Style Inventory`))
  (bind _radial_inventory_style_1 (`self.Radial Inventory Style 1`))
  (bind _radial_inventory_style_2 (`self.Radial Inventory Style 2`))
  (bind _radial_inventory_style_3 (`self.Radial Inventory Style 3`))
  (bind _deus_ex_style_inventory (`self.Deus EX Style Inventory`))
  (bind _dead_space_style_inventory (`self.Dead Space Style Inventory`))
  ;[1 0 0] Close Inventory
  (`|ExecutionSequence`
    (:`then_0`
      (`/Engine/EditorBlueprintResources/StandardMacros.IsValid` _half_life_alyx_style_inventory
        (:`Is Valid`
          (`/Game/VR_Inventorys/Inventory_Menus/HLA_Inventory/BP_HLA_Inventory.OnDisappear` _half_life_alyx_style_inventory)
          (`Actor.K2_SetActorLocation` _half_life_alyx_style_inventory (0.0 0.0 -500.0) false true))))
    (:`then_1`
      (`/Engine/EditorBlueprintResources/StandardMacros.IsValid` _dead_space_style_inventory
        (:`Is Valid`
          (`/Game/VR_Inventorys/Inventory_Menus/2D_Type_Inventorys/BP_DS_Inventory_Menu.On Close Menu` _dead_space_style_inventory)
          (`Actor.K2_SetActorLocation` _dead_space_style_inventory (0.0 0.0 -500.0) false true))))
    (:`then_2`
      (`/Engine/EditorBlueprintResources/StandardMacros.IsValid` _deus_ex_style_inventory
        (:`Is Valid`
          (`/Game/VR_Inventorys/Inventory_Menus/2D_Type_Inventorys/BP_Deus_Inventory.On Close Menu` _deus_ex_style_inventory)
          (`Actor.K2_SetActorLocation` _deus_ex_style_inventory (0.0 0.0 -500.0) false true))))
    (:`then_3`
      (`/Engine/EditorBlueprintResources/StandardMacros.IsValid` _radial_inventory_style_1
        (:`Is Valid`
          (`/Game/VR_Inventorys/Inventory_Menus/Radial_Inventorys/BP_Radial_Ring_Inventory.OnDisappear` _radial_inventory_style_1)
          (`KismetSystemLibrary.Delay` 1.5)
          (`Actor.K2_SetActorLocation` _radial_inventory_style_1 (0.0 0.0 -500.0) false true))))
    (:`then_4`
      (`/Engine/EditorBlueprintResources/StandardMacros.IsValid` _radial_inventory_style_2
        (:`Is Valid`
          (`/Game/VR_Inventorys/Inventory_Menus/Radial_Inventorys/BP_Radial_Ring_Inventory_2.OnDisappear` _radial_inventory_style_2)
          (`KismetSystemLibrary.Delay` 1.5)
          (`Actor.K2_SetActorLocation` _radial_inventory_style_2 (0.0 0.0 -500.0) false true))))
    (:`then_5`
      (`/Engine/EditorBlueprintResources/StandardMacros.IsValid` _radial_inventory_style_3
        (:`Is Valid`
          (`/Game/VR_Inventorys/Inventory_Menus/Radial_Inventorys/BP_Radial_Ring_Inventory_3.OnDisappear` _radial_inventory_style_3)
          (`KismetSystemLibrary.Delay` 1.5)
          (`Actor.K2_SetActorLocation` _radial_inventory_style_3 (0.0 0.0 -500.0) false true))))))

(event `Call Inventory`
  (params (`Players VR Hand` :type "SkeletalMeshComponent Object Reference") (`Players VR Camera` :type "CameraComponent Object Reference") (`Any scene Component` :type "SceneComponent Object Reference") (Selection :type "/Game/VR_Inventorys/Blueprints/Enum_Inventory_Menu_Type_enum Enum" :default "NewEnumerator0"))
  (bind _returnvalue (`SceneComponent.K2_GetComponentLocation` `Any scene Component`))
  (bind _radial_inventory_style_2 (`self.Radial Inventory Style 2`))
  (bind _radial_inventory_style_3 (`self.Radial Inventory Style 3`))
  (bind _half_life_alyx_style_inventory (`self.Half Life Alyx Style Inventory`))
  (bind _deus_ex_style_inventory (`self.Deus EX Style Inventory`))
  (bind _dead_space_style_inventory (`self.Dead Space Style Inventory`))
  (bind _radial_inventory_style_1 (`self.Radial Inventory Style 1`))
  (bind _returnvalue_2 (+ (`SceneComponent.K2_GetComponentLocation` `Players VR Camera`) (* (`SceneComponent.GetForwardVector` `Players VR Camera`) 70.0)))
  (bind _returnvalue_3 (+ (`SceneComponent.K2_GetComponentLocation` `Players VR Hand`) (* (`SceneComponent.GetRightVector` `Players VR Hand`) 30.0)))
  ;[1 0.9023 0] Open Inventory
  (switch `/Game/VR_Inventorys/Blueprints/Enum_Inventory_Menu_Type_enum` Selection
    (:`NewEnumerator0`
      (`/Engine/EditorBlueprintResources/StandardMacros.IsValid` _half_life_alyx_style_inventory
        (:`Is Valid`
          (`Actor.K2_SetActorLocation` _half_life_alyx_style_inventory _returnvalue_3 false true)
          (`/Game/VR_Inventorys/Inventory_Menus/HLA_Inventory/BP_HLA_Inventory.Appear` _half_life_alyx_style_inventory))
        (:`Is Not Valid`
          (bind _returnvalue_4 (`|SpawnActorFromClass` "/Game/VR_Inventorys/Inventory_Menus/HLA_Inventory/BP_HLA_Inventory.BP_HLA_Inventory_C" (`KismetMathLibrary.MakeTransform` _returnvalue_3) "Undefined" "OverrideRootScale" null null))
          (set `self.Half Life Alyx Style Inventory` _returnvalue_4))))
    (:`NewEnumerator1`
      ;[0.01687 0.1593 1] Dead Space 2D Style
      (`/Engine/EditorBlueprintResources/StandardMacros.IsValid` _dead_space_style_inventory
        (:`Is Valid`
          (`Actor.K2_SetActorLocation` _dead_space_style_inventory _returnvalue_2 false true)
          (`/Game/VR_Inventorys/Inventory_Menus/2D_Type_Inventorys/BP_DS_Inventory_Menu.On Open Menu` _dead_space_style_inventory))
        (:`Is Not Valid`
          (bind _returnvalue_5 (`|SpawnActorFromClass` "/Game/VR_Inventorys/Inventory_Menus/2D_Type_Inventorys/BP_DS_Inventory_Menu.BP_DS_Inventory_Menu_C" (`KismetMathLibrary.MakeTransform` _returnvalue_2) "Undefined" "OverrideRootScale" null null))
          (set `self.Dead Space Style Inventory` _returnvalue_5))))
    (:`NewEnumerator2`
      ;[0.7865 0.3654 0 0.587] Deux EX style 2D Inventory
      (`/Engine/EditorBlueprintResources/StandardMacros.IsValid` _radial_inventory_style_1
        (:`Is Valid`
          (`Actor.K2_SetActorLocation` _radial_inventory_style_1 _returnvalue false true)
          (`/Game/VR_Inventorys/Inventory_Menus/Radial_Inventorys/BP_Radial_Ring_Inventory.Appear` _radial_inventory_style_1))
        (:`Is Not Valid`
          (bind _returnvalue_6 (`|SpawnActorFromClass` "/Game/VR_Inventorys/Inventory_Menus/Radial_Inventorys/BP_Radial_Ring_Inventory.BP_Radial_Ring_Inventory_C" (`KismetMathLibrary.MakeTransform` _returnvalue) "Undefined" "OverrideRootScale" null null))
          (set `self.Radial Inventory Style 1` _returnvalue_6))))
    (:`NewEnumerator3`
      ;[0.7865 0.3654 0 0.587] Deux EX style 2D Inventory
      (`/Engine/EditorBlueprintResources/StandardMacros.IsValid` _deus_ex_style_inventory
        (:`Is Valid`
          (`Actor.K2_SetActorLocation` _deus_ex_style_inventory _returnvalue_2 false true)
          (`/Game/VR_Inventorys/Inventory_Menus/2D_Type_Inventorys/BP_Deus_Inventory.On Open Menu` _deus_ex_style_inventory))
        (:`Is Not Valid`
          (bind _returnvalue_7 (`|SpawnActorFromClass` "/Game/VR_Inventorys/Inventory_Menus/2D_Type_Inventorys/BP_Deus_Inventory.BP_Deus_Inventory_C" (`KismetMathLibrary.MakeTransform` _returnvalue_2 (struct) (0.6 0.6 0.6)) "Undefined" "OverrideRootScale" null null))
          (set `self.Deus EX Style Inventory` _returnvalue_7))))
    (:`NewEnumerator4`
      ;[0.7865 0.3654 0 0.587] Radial 2
      (`/Engine/EditorBlueprintResources/StandardMacros.IsValid` _radial_inventory_style_2
        (:`Is Valid`
          (`Actor.K2_SetActorLocation` _radial_inventory_style_2 _returnvalue false true)
          (`/Game/VR_Inventorys/Inventory_Menus/Radial_Inventorys/BP_Radial_Ring_Inventory_2.Appear` _radial_inventory_style_2))
        (:`Is Not Valid`
          (bind _returnvalue_8 (`|SpawnActorFromClass` "/Game/VR_Inventorys/Inventory_Menus/Radial_Inventorys/BP_Radial_Ring_Inventory_2.BP_Radial_Ring_Inventory_2_C" (`KismetMathLibrary.MakeTransform` _returnvalue) "Undefined" "OverrideRootScale" null null))
          (set `self.Radial Inventory Style 2` _returnvalue_8))))
    (:`NewEnumerator5`
      ;[0.7865 0.3654 0 0.587] Radial 3
      (`/Engine/EditorBlueprintResources/StandardMacros.IsValid` _radial_inventory_style_3
        (:`Is Valid`
          (`Actor.K2_SetActorLocation` _radial_inventory_style_3 _returnvalue false true)
          (`/Game/VR_Inventorys/Inventory_Menus/Radial_Inventorys/BP_Radial_Ring_Inventory_3.Appear` _radial_inventory_style_3))
        (:`Is Not Valid`
          (bind _returnvalue_9 (`|SpawnActorFromClass` "/Game/VR_Inventorys/Inventory_Menus/Radial_Inventorys/BP_Radial_Ring_Inventory_3.BP_Radial_Ring_Inventory_3_C" (`KismetMathLibrary.MakeTransform` _returnvalue) "Undefined" "OverrideRootScale" null null))
          (set `self.Radial Inventory Style 3` _returnvalue_9))))))