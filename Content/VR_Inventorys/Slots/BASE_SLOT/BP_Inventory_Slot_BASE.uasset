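; Base VR inventory slot actor that stores a held item and hands it back to a motion controller on grab.
; A SlotConfiguration struct sets its look, accepted type, holster mode, hover feedback and optional auto-spawned item, whose type overrides the slot's.
; Quick store attaches matching items using grab-component transforms, flashing red on rejection; AutoStore skips those checks.
; Timelines animate menu appearance and hover scaling, alongside rotation, opacity, haptics and sound.
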(event `Detect Interaction`
  (params (`Held Object` :type "/Game/VR_Inventorys/Blueprints/BP_VRM_GrabComponent Object Reference") (`Motion Controller` :type "MotionControllerComponent Object Reference"))
  (bind (_slot_configuration_dontshowouterring _slot_configuration_dontshowslottext _slot_configuration_dontshowemptysloticon _slot_configuration_sizescalingoninteraction _slot_configuration_opacityscalingoninteraction _slot_configuration_rotationoninteraction _slot_configuration_slotcolor _slot_configuration_outerringcolor _slot_configuration_slottype) (break `/Game/VR_Inventorys/Blueprints/Struct_Slot_Config` (`self.Slot configuration`)))
  (bind (_slot_configuration_dontshowouterring_2 _slot_configuration_dontshowslottext_2 _slot_configuration_dontshowemptysloticon_2 _slot_configuration_sizescalingoninteraction_2 _slot_configuration_opacityscalingoninteraction_2 _slot_configuration_rotationoninteraction_2 _slot_configuration_slotcolor_2 _slot_configuration_outerringcolor_2 _slot_configuration_slottype_2 _slot_configuration_holster _slot_configuration_autospawnitem _slot_configuration_slottedhapticeffect _slot_configuration_interactionhapticeffect) (break `/Game/VR_Inventorys/Blueprints/Struct_Slot_Config` (`self.Slot configuration`)))
  ;[0 0 0] Hand Interaction
  (set `self.Motion Controller ref` `Motion Controller`)
  ;;[0 0 0] Held Item Detection
  (`/Engine/EditorBlueprintResources/StandardMacros.IsValid` `Held Object` ; Is Holding Object?
    (:`Is Valid`
      (set `self.Detected Item` `Held Object`)
      (if (not (`self.Slot in Use`))
        ;;;[1 1 1] Check Item is correct slot type
        (if (`|EnumEquality` (`/Game/VR_Inventorys/Blueprints/BP_VRM_GrabComponent.SlotType` (`self.Detected Item`)) _slot_configuration_slottype)
          ;;[0.2917 0 1] FX
          (`self.Play Haptic Effect On correct hand` _slot_configuration_interactionhapticeffect 1.0 :!label _label)
          (`|ExecutionSequence`
            (:`then_0`
              (if _slot_configuration_sizescalingoninteraction_2
                (`self.Scale Up Slot`)))
            (:`then_1`
              (if _slot_configuration_opacityscalingoninteraction_2
                (`MaterialInstanceDynamic.SetScalarParameterValue` (`self.Slot Dynamic Mat`) "MinOpacity" 1.0)))
            (:`then_2`
              (if _slot_configuration_rotationoninteraction_2
                (`self.Rotate Slot`)))))))
    (:`Is Not Valid`
      ;;[0 0 0] Empty Hand detection
      (if (`self.Slot in Use`)
        (goto _label)))))

(event `self.ReceiveBeginPlay`
  (bind (_slot_configuration_dontshowouterring _slot_configuration_dontshowslottext _slot_configuration_dontshowemptysloticon _slot_configuration_sizescalingoninteraction _slot_configuration_opacityscalingoninteraction _slot_configuration_rotationoninteraction _slot_configuration_slotcolor _slot_configuration_outerringcolor _slot_configuration_slottype _slot_configuration_holster _slot_configuration_autospawnitem _slot_configuration_slottedhapticeffect _slot_configuration_interactionhapticeffect) (break `/Game/VR_Inventorys/Blueprints/Struct_Slot_Config` (`self.Slot configuration`)))
  (set `self.Current 3D Scale` (`SceneComponent.RelativeScale3D` (`self.Slot mesh`)))
  ;[1 1 1] Use Dynamic Material, Allows Control of  Material Paramaters
  (bind _returnvalue (`PrimitiveComponent.CreateDynamicMaterialInstance` (`self.Slot mesh`) 0 null "None"))
  (set `self.Slot Dynamic Mat` _returnvalue)
  (bind _returnvalue_2 (`PrimitiveComponent.CreateDynamicMaterialInstance` (`self.Ring mesh`) 0 null "None"))
  (set `self.Ring Dynamic Mat` _returnvalue_2)
  (`PrimitiveComponent.SetMaterial` (`self.Slot mesh`) 0 (`self.Slot Dynamic Mat`))
  (`PrimitiveComponent.SetMaterial` (`self.Ring mesh`) 0 (`self.Ring Dynamic Mat`))
  ;[0.8853 1 0] Slot CONFIG
  (`self.Slot  config` _slot_configuration_dontshowouterring _slot_configuration_dontshowemptysloticon _slot_configuration_dontshowslottext _slot_configuration_slotcolor _slot_configuration_outerringcolor _slot_configuration_opacityscalingoninteraction _slot_configuration_slottype _slot_configuration_holster _slot_configuration_autospawnitem _slot_configuration_interactionhapticeffect _slot_configuration_slottedhapticeffect)
  ;[1 1 1] Set up Rotation mesh
  (`MovementComponent.SetUpdatedComponent` (`self.RotatingMovement`) (`self.Slot mesh`)))

(event `Detect End Interaction`
  (params (`Held Object` :type "/Game/VR_Inventorys/Blueprints/BP_VRM_GrabComponent Object Reference"))
  (bind (_slot_configuration_dontshowouterring _slot_configuration_dontshowslottext _slot_configuration_dontshowemptysloticon _slot_configuration_sizescalingoninteraction _slot_configuration_opacityscalingoninteraction _slot_configuration_rotationoninteraction) (break `/Game/VR_Inventorys/Blueprints/Struct_Slot_Config` (`self.Slot configuration`)))
  ;[0 0 0] Hand Interaction
  ;;[1 1 1] Item Leaves Slot
  (`/Engine/EditorBlueprintResources/StandardMacros.IsValid` `Held Object`
    (:`Is Valid`
      (if (== `Held Object` (`self.Detected Item`))
        (set `self.Detected Item` null) ; Cleared!
        (if (`self.Slot in Use`)
          ;;[0.2917 0 1] FX
          (`|ExecutionSequence` :!label _label_2
            (:`then_0`
              (if _slot_configuration_sizescalingoninteraction
                (`self.Scale Down Slot`)))
            (:`then_1`
              (if _slot_configuration_rotationoninteraction :!label _label_3
                (`self.Stop Slot rotation`))))
          (else
            (`|ExecutionSequence` :!label _label_4
              (:`then_0`
                (if _slot_configuration_opacityscalingoninteraction
                  (`MaterialInstanceDynamic.SetScalarParameterValue` (`self.Slot Dynamic Mat`) "MinOpacity" 0.1)))
              (:`then_1`
                (goto _label_3))
              (:`then_2`
                (if _slot_configuration_sizescalingoninteraction
                  (`self.Scale Down Slot`))))))))
    (:`Is Not Valid`
      (if (`self.Slot in Use`)
        (goto _label_2)
        (else
          (goto _label_4))))))

(event `self.Detect Box.OnComponentBeginOverlap`
  (params (OverlappedComponent :type "PrimitiveComponent Object Reference") (OtherActor :type "Actor Object Reference") (OtherComp :type "PrimitiveComponent Object Reference") (OtherBodyIndex :type Integer) (bFromSweep :type Boolean) (SweepResult :type "HitResult Structure (by ref)"))
  ;[0 0 0] Hand Interaction
)

(event `self.InventoryQuickGrab`
  (params (`Motion Controller` :type "MotionControllerComponent Object Reference"))
  (bind _primitive_component (`self.Primitive Component`))
  (bind (_slot_configuration_dontshowouterring _slot_configuration_dontshowslottext _slot_configuration_dontshowemptysloticon) (break `/Game/VR_Inventorys/Blueprints/Struct_Slot_Config` (`self.Slot configuration`)))
  ;[1 1 1] Quick Grab Slotted Item
  (bind _slotted_actor (`self.Slotted Actor`)
    (:`then`
      (`/Game/VR_Inventorys/Blueprints/BP_VRM_GrabComponent.Try Grab` (`self.GetComponentByClass` _slotted_actor "/Game/VR_Inventorys/Blueprints/BP_VRM_GrabComponent.BP_VRM_GrabComponent_C") `Motion Controller`)
      (`self.SetActorScale3D` (`self.Slotted Actor`) (`self.Actors Original scale`)) ; Set actor to correct scale before grabbing
      (`/Engine/EditorBlueprintResources/StandardMacros.IsValid` _primitive_component
        (:`Is Valid`
          (`PrimitiveComponent.SetCollisionResponseToAllChannels` _primitive_component "ECR_Block") ; Prevent collision issues when slotted
          (`PrimitiveComponent.SetCastShadow` _primitive_component true) ; dont want Slotted Items casting shadows
          (`|ExecutionSequence`
            (:`then_0`
              (set `self.Slot in Use` false)
              (if (not _slot_configuration_dontshowemptysloticon)
                (`SceneComponent.SetHiddenInGame` (`self.Empty Icon`) false false))
              (`self.Update Slot Opacity` 0.1)
              (set `/Game/VR_Inventorys/Blueprints/BP_VRM_GrabComponent.Slotted?` false (`self.Slotted Actors Grab Component`)))
            (:`then_1`
              ;;[1 1 1] Clear refs
              (set `self.Primitive Component` null)
              (set `self.Skel Mesh Component` null)
              (set `self.Static Mesh Component` null)
              (set `self.Slotted Actor` null)
              (set `self.Slotted Actors Grab Component` null))))))
    (:`else`)))

(event `self.ReceiveTick`
  (params (DeltaSeconds :type "Float (single-precision)"))
  ;[0.1788 0.1788 0.1788] TESTING TOOL ( NOT FOR ACTUAL USE)
  ;;[1 0.3136 0] Tester
)

(event `self.Detect Box.OnComponentEndOverlap`
  (params (OverlappedComponent :type "PrimitiveComponent Object Reference") (OtherActor :type "Actor Object Reference") (OtherComp :type "PrimitiveComponent Object Reference") (OtherBodyIndex :type Integer))
  ;[0 0 0] Hand Interaction
)

(event `Wrong slot Timer`
  (bind (_slot_configuration_dontshowouterring _slot_configuration_dontshowslottext _slot_configuration_dontshowemptysloticon _slot_configuration_sizescalingoninteraction _slot_configuration_opacityscalingoninteraction _slot_configuration_rotationoninteraction _slot_configuration_slotcolor) (break `/Game/VR_Inventorys/Blueprints/Struct_Slot_Config` (`self.Slot configuration`)))
  ;[0.009375 0.005342 0.005409] Slot  / Store Actor
  ;;[1 0.002493 0] Trun Red Or Any Other Colour On wrong slot type, for The set time
  (`MaterialInstanceDynamic.SetVectorParameterValue` (`self.Slot Dynamic Mat`) "Color" _slot_configuration_slotcolor) ; Restore to Original Color
  (`KismetSystemLibrary.K2_ClearAndInvalidateTimerHandle` (stale `self.InventoryQuickStore` _returnvalue_3)))

(event `self.InventoryQuickStore`
  (params (`Slot Type` :type "/Game/VR_Inventorys/Blueprints/Enum_Inventory_slotType Enum" :default "NewEnumerator0") (ACTOR :type "Actor Object Reference") (`Skeletal Mesh` :type "SkeletalMeshComponent Object Reference") (`Static mesh` :type "StaticMeshComponent Object Reference") (`Primitive Component` :type "PrimitiveComponent Object Reference") (`Pawn Held Component Ref ` :type "/Game/VR_Inventorys/Blueprints/BP_VRM_GrabComponent Object Reference") (`Motion Controller` :type "MotionControllerComponent Object Reference"))
  (bind (_slot_configuration_dontshowouterring _slot_configuration_dontshowslottext _slot_configuration_dontshowemptysloticon _slot_configuration_sizescalingoninteraction _slot_configuration_opacityscalingoninteraction _slot_configuration_rotationoninteraction _slot_configuration_slotcolor _slot_configuration_outerringcolor _slot_configuration_slottype _slot_configuration_holster _slot_configuration_autospawnitem _slot_configuration_slottedhapticeffect _slot_configuration_interactionhapticeffect _slot_configuration_slottedsoundeffect) (break `/Game/VR_Inventorys/Blueprints/Struct_Slot_Config` (`self.Slot configuration`)))
  (bind _slotted_actor (`self.Slotted Actor`))
  (bind (_slot_configuration_dontshowouterring_2 _slot_configuration_dontshowslottext_2 _slot_configuration_dontshowemptysloticon_2 _slot_configuration_sizescalingoninteraction_2 _slot_configuration_opacityscalingoninteraction_2 _slot_configuration_rotationoninteraction_2 _slot_configuration_slotcolor_2 _slot_configuration_outerringcolor_2 _slot_configuration_slottype_2 _slot_configuration_holster_2) (break `/Game/VR_Inventorys/Blueprints/Struct_Slot_Config` (`self.Slot configuration`)))
  (bind (_slot_configuration_dontshowouterring_3 _slot_configuration_dontshowslottext_3 _slot_configuration_dontshowemptysloticon_3 _slot_configuration_sizescalingoninteraction_3 _slot_configuration_opacityscalingoninteraction_3 _slot_configuration_rotationoninteraction_3 _slot_configuration_slotcolor_3 _slot_configuration_outerringcolor_3 _slot_configuration_slottype_3 _slot_configuration_holster_3 _slot_configuration_autospawnitem_2 _slot_configuration_slottedhapticeffect_2) (break `/Game/VR_Inventorys/Blueprints/Struct_Slot_Config` (`self.Slot configuration`)))
  (bind _primitive_component (`self.Primitive Component`))
  (bind _returnvalue (`self.GetComponentByClass` (`self.Slotted Actor`) "/Game/VR_Inventorys/Blueprints/BP_VRM_GrabComponent.BP_VRM_GrabComponent_C"))
  (bind _returnvalue_2 (`self.GetComponentByClass` _slotted_actor "/Game/VR_Inventorys/Blueprints/BP_VRM_GrabComponent.BP_VRM_GrabComponent_C"))
  ;[0.009375 0.005342 0.005409] Slot  / Store Actor
  ;;[0.01576 1 0] Quick store
  ;;;[0 0 0] Set Refs
  (set `self.Item Slot Type` `Slot Type`)
  (set `self.Slotted Actor` ACTOR)
  (set `self.Skel Mesh Component` `Skeletal Mesh`)
  (set `self.Static Mesh Component` `Static mesh`)
  (set `self.Primitive Component` `Primitive Component`)
  (set `self.Motion Controller ref` `Motion Controller`)
  (set `self.Slotted Actors Grab Component` _returnvalue) ; Create Ref to slotted actors Grab Component
  (set `self.Actors Original scale` (`/Game/VR_Inventorys/Blueprints/BP_VRM_GrabComponent.Default World scale` _returnvalue)) ; Used To restore actor to proper size on Slot grab
  (if (`self.Slot in Use`)
    ;;[1 0.002493 0] Trun Red Or Any Other Colour On wrong slot type, for The set time
    (bind _returnvalue_3 (`KismetSystemLibrary.K2_SetTimerDelegate` (delegate `Wrong slot Timer`) 1.0 :!label _label_5))
    (`MaterialInstanceDynamic.SetVectorParameterValue` (`self.Slot Dynamic Mat`) "Color" (struct :`R` 1.0 :`A` 1.0))
    (`/Game/VR_Inventorys/Blueprints/BP_VRM_GrabComponent.Try Release` (`self.Slotted Actors Grab Component`))
    (else
      ;;[0.1982 1 0] Slot Type Check
      (if (== (`self.Item Slot Type`) _slot_configuration_slottype_2)
        (`/Engine/EditorBlueprintResources/StandardMacros.IsValid` _primitive_component
          (:`Is Valid`
            (`PrimitiveComponent.SetCollisionResponseToAllChannels` _primitive_component "ECR_Ignore") ; Prevent collision issues when slotted
            (`PrimitiveComponent.SetCastShadow` _primitive_component false) ; dont want Slotted Items casting shadows
            (`self.K2_AttachToComponent` (`self.Slotted Actor`) (`self.AttachPoint`) "None" "SnapToTarget" "SnapToTarget" "KeepWorld" true)
            (if _slot_configuration_holster_2
              (`self.K2_SetActorRelativeTransform` _slotted_actor (`/Game/VR_Inventorys/Blueprints/BP_VRM_GrabComponent.Holster Transform` _returnvalue_2) false false)
              (else
                (`self.K2_SetActorRelativeTransform` _slotted_actor (`/Game/VR_Inventorys/Blueprints/BP_VRM_GrabComponent.Slotted Transfrom` _returnvalue_2) false false :!label _label_6)
                (if (not _slot_configuration_dontshowemptysloticon_3)
                  (`SceneComponent.SetHiddenInGame` (`self.Empty Icon`) true false))
                (`self.Play Haptic Effect On correct hand` _slot_configuration_slottedhapticeffect_2 1.0)
                (set `self.Slot in Use` true)
                ;;[1 1 1] Set slot to default colour when in use (to compensate for detect grab component slot type   changing the color to green.
                (`MaterialInstanceDynamic.SetVectorParameterValue` (`self.Slot Dynamic Mat`) "Color" _slot_configuration_slotcolor)
                (`self.Update Slot Opacity` 1.0)
                (set `/Game/VR_Inventorys/Blueprints/BP_VRM_GrabComponent.Slotted?` true (`self.Slotted Actors Grab Component`))
                (`self.Slot Sound` _slot_configuration_slottedsoundeffect)))))
        (else
          (goto _label_5))))))

(event `self.Auto Store`
  (params (`Slot type` :type "/Game/VR_Inventorys/Blueprints/Enum_Inventory_slotType Enum" :default "NewEnumerator0") (ACTOR :type "Actor Object Reference") (`Skeletal Mesh` :type "SkeletalMeshComponent Object Reference") (`Static mesh` :type "StaticMeshComponent Object Reference") (`Primitive Component` :type "PrimitiveComponent Object Reference") (`Pawn Held Component Ref ` :type "/Game/VR_Inventorys/Blueprints/BP_VRM_GrabComponent Object Reference") (`Motion Controller` :type "MotionControllerComponent Object Reference"))
  (bind _primitive_component (`self.Primitive Component`))
  (bind _returnvalue (`self.GetComponentByClass` (`self.Slotted Actor`) "/Game/VR_Inventorys/Blueprints/BP_VRM_GrabComponent.BP_VRM_GrabComponent_C"))
  ;[0.009375 0.005342 0.005409] Slot  / Store Actor
  ;;[0 0.4304 1] Auto - store
  (set `self.Item Slot Type` `Slot type`)
  ;;;[0 0 0] Set Refs
  (set `self.Slotted Actor` ACTOR)
  (set `self.Skel Mesh Component` `Skeletal Mesh`)
  (set `self.Static Mesh Component` `Static mesh`)
  (set `self.Primitive Component` `Primitive Component`)
  (set `self.Motion Controller ref` `Motion Controller`)
  (set `self.Slotted Actors Grab Component` _returnvalue) ; Create Ref to slotted actors Grab Component
  (set `self.Actors Original scale` (`/Game/VR_Inventorys/Blueprints/BP_VRM_GrabComponent.Default World scale` _returnvalue)) ; Used To restore actor to proper size on Slot grab
  (`/Engine/EditorBlueprintResources/StandardMacros.IsValid` _primitive_component
    (:`Is Valid`
      (`PrimitiveComponent.SetCollisionResponseToAllChannels` _primitive_component "ECR_Ignore") ; Prevent collision issues when slotted
      (`PrimitiveComponent.SetCastShadow` _primitive_component false) ; dont want Slotted Items casting shadows
      (`self.K2_AttachToComponent` (`self.Slotted Actor`) (`self.AttachPoint`) "None" "SnapToTarget" "SnapToTarget" "KeepWorld" true)
      (goto _label_6))))

(event `Appear`
  ;[1 1 1] On Appear Scale Up Slots ( Initial Anim Transition FOR Inventory Menu Spawn )
  (`self.SetActorHiddenInGame` false)
  (bind (_direction _lerp) (`Timeline|Scale UP` :!via `PlayFromStart` :!label _label_7)
    (:`Update`
      ;;[1 1 1] Scale
      (`self.SetActorRelativeScale3D` (`KismetMathLibrary.VLerp` (0.0 0.0 0.0) (1.0 1.0 1.0) _lerp)))
    (:`Finished`
      ;;[1 1 1] Hide after scale down
      (switch `ETimelineDirection` _direction
        (:`Backward`
          (`self.SetActorHiddenInGame` true))))))

(event `Scale Up Slot`
  ;[1 1 1] Potential Slot Interaction when Hand Hover over Occupied slot
  (bind (_direction _lerp) (`Timeline|Hand Hover Slot Interaction` :!label _label_8)
    (:`Update`
      (`SceneComponent.SetRelativeScale3D` (`self.Slot mesh`) (`KismetMathLibrary.VLerp` (`self.Current 3D Scale`) (0.2 0.2 0.2) _lerp)))))

(event `Disappear`
  ;[1 1 1] On Appear Scale Up Slots ( Initial Anim Transition FOR Inventory Menu Spawn )
  (goto _label_7 :!via `ReverseFromEnd`))

(event `Scale Down Slot`
  ;[1 1 1] Potential Slot Interaction when Hand Hover over Occupied slot
  (goto _label_8 :!via `Reverse`))

(event `Rotate Slot`
  ;[1 1 1] Slot rotatation
  (`ActorComponent.Activate` (`self.RotatingMovement`) false))

(event `Slot Sound`
  (params (Sound :type "SoundBase Object Reference"))
  ;[1 1 1] Play a Sound at slot location
  (`GameplayStatics.SpawnSoundAtLocation` Sound (`SceneComponent.K2_GetComponentLocation` (`self.AttachPoint`)) (struct) 1.0 1.0 0.0 null null))

(event `Stop Slot rotation`
  ;[1 1 1] Slot rotatation
  (`ActorComponent.Deactivate` (`self.RotatingMovement`)))

(fn `AutoSpawn Item In SLOT`
  (params (`Spawn Item` :type "Actor Class Reference"))
  (bind (_slot_configuration_dontshowouterring _slot_configuration_dontshowslottext _slot_configuration_dontshowemptysloticon _slot_configuration_sizescalingoninteraction _slot_configuration_opacityscalingoninteraction _slot_configuration_rotationoninteraction _slot_configuration_slotcolor _slot_configuration_outerringcolor _slot_configuration_slottype _slot_configuration_holster _slot_configuration_autospawnitem _slot_configuration_slottedhapticeffect _slot_configuration_interactionhapticeffect _slot_configuration_slottedsoundeffect) (break `/Game/VR_Inventorys/Blueprints/Struct_Slot_Config` (`self.Slot configuration`)))
  (bind _returnvalue (`|SpawnActorFromClass` `Spawn Item` (`KismetMathLibrary.MakeTransform` (0.0 0.0 0.0)) "AlwaysSpawn" "OverrideRootScale" null null))
  (bind _returnvalue_2 (`self.GetComponentByClass` _returnvalue "/Game/VR_Inventorys/Blueprints/BP_VRM_GrabComponent.BP_VRM_GrabComponent_C"))
  (bind _slottype (`/Game/VR_Inventorys/Blueprints/BP_VRM_GrabComponent.SlotType` _returnvalue_2))
  ;[0.1549 0 1] Automatically Change the slot type to match The Auto spawned Actor's Slot type
  (set `self.Slot configuration` (make `/Game/VR_Inventorys/Blueprints/Struct_Slot_Config` _slot_configuration_dontshowouterring _slot_configuration_dontshowslottext _slot_configuration_dontshowemptysloticon _slot_configuration_sizescalingoninteraction _slot_configuration_opacityscalingoninteraction _slot_configuration_rotationoninteraction _slot_configuration_slotcolor _slot_configuration_outerringcolor _slottype _slot_configuration_holster _slot_configuration_autospawnitem _slot_configuration_slottedhapticeffect _slot_configuration_interactionhapticeffect _slot_configuration_slottedsoundeffect))
  (`self.InventoryQuickStore` _slottype _returnvalue null null (`self.GetComponentByClass` _returnvalue "/Script/Engine.PrimitiveComponent") _returnvalue_2))

(fn `Play Haptic Effect On correct hand`
  (params (`Haptic Effect` :type "HapticFeedbackEffect_Base Object Reference") (Scale :type "Float (single-precision)"))
  (bind _motion_controller_ref (`self.Motion Controller ref`) ; Only Play effect If MC is Valid
    (:`then`
      (`PlayerController.PlayHapticEffect` (`GameplayStatics.GetPlayerController` 0) `Haptic Effect` (select `bool` (== (`MotionControllerComponent.MotionSource` _motion_controller_ref) "Left") :`false` "Right" :`true` "Left" :!type "EControllerHand Enum") Scale false))
    (:`else`)))

(fn `Slot  config`
  (params (`Hide Outer ring ` :type Boolean) (`Hide Empty slot Icon` :type Boolean) (`Hide Slot text` :type Boolean) (`Slot color` :type "LinearColor Structure") (`Outer Ring Color` :type "LinearColor Structure") (`Slot Mat Opacity` :type Boolean) (`Slot Type` :type "/Game/VR_Inventorys/Blueprints/Enum_Inventory_slotType Enum" :default "NewEnumerator0") (Holster :type Boolean) (`AutoSpawn type` :type "/Game/VR_Inventorys/Blueprints/Enum_Autospawn Enum" :default "NewEnumerator0") (`Slot Detect Haptic` :type "HapticFeedbackEffect_Base Object Reference") (`Store Item Haptic` :type "HapticFeedbackEffect_Base Object Reference"))
  (bind _slot_dynamic_mat (`self.Slot Dynamic Mat`))
  (bind _ring_dynamic_mat (`self.Ring Dynamic Mat`))
  (`|ExecutionSequence`
    (:`then_0`
      (`SceneComponent.SetHiddenInGame` (`self.Ring mesh`) `Hide Outer ring ` false) ; Hide Outer Ring
    )
    (:`then_1`
      (`SceneComponent.SetHiddenInGame` (`self.Empty Icon`) `Hide Empty slot Icon` false) ; Hide Empty Icon
    )
    (:`then_2`
      (`SceneComponent.SetHiddenInGame` (`self.TextRender`) `Hide Slot text` false) ; Hide Slot Info Text
    )
    (:`then_3`
      (`/Engine/EditorBlueprintResources/StandardMacros.IsValid` _slot_dynamic_mat
        (:`Is Valid`
          (`MaterialInstanceDynamic.SetVectorParameterValue` _slot_dynamic_mat "Color" `Slot color`))))
    (:`then_4`
      (`/Engine/EditorBlueprintResources/StandardMacros.IsValid` _ring_dynamic_mat
        (:`Is Valid`
          (`MaterialInstanceDynamic.SetVectorParameterValue` _ring_dynamic_mat "Color" `Outer Ring Color`))))
    (:`then_5`
      (if `Slot Mat Opacity`
        (`MaterialInstanceDynamic.SetScalarParameterValue` (`self.Slot Dynamic Mat`) "MinOpacity" 0.1)))
    (:`then_6`
      (switch `/Game/VR_Inventorys/Blueprints/Enum_Autospawn` `AutoSpawn type`
        (:`NewEnumerator1`
          (`self.AutoSpawn Item In SLOT` "/Game/VR_Inventorys/Items/BP_VR_Pistol.BP_VR_Pistol_C"))
        (:`NewEnumerator2`
          (`self.AutoSpawn Item In SLOT` "/Game/VR_Inventorys/Items/BP_ShotGun.BP_ShotGun_C"))
        (:`NewEnumerator3`
          (`self.AutoSpawn Item In SLOT` "/Game/VR_Inventorys/Items/BP_Rifle.BP_Rifle_C"))
        (:`NewEnumerator13`
          (`self.AutoSpawn Item In SLOT` "/Game/VR_Inventorys/Items/BP_Rifle2.BP_Rifle2_C"))
        (:`NewEnumerator4`
          (`self.AutoSpawn Item In SLOT` "/Game/VR_Inventorys/Items/BP_Grenade.BP_Grenade_C"))
        (:`NewEnumerator5`
          (`self.AutoSpawn Item In SLOT` "/Game/VR_Inventorys/Items/BP_Small_Health.BP_Small_Health_C"))
        (:`NewEnumerator6`
          (`self.AutoSpawn Item In SLOT` "/Game/VR_Inventorys/Items/BP_Large_Health.BP_Large_Health_C"))
        (:`NewEnumerator7`
          (`self.AutoSpawn Item In SLOT` "/Game/VR_Inventorys/Items/BP_Machette.BP_Machette_C"))
        (:`NewEnumerator8`
          (`self.AutoSpawn Item In SLOT` "/Game/VR_Inventorys/Items/BP_Machette_2.BP_Machette_2_C"))
        (:`NewEnumerator9`
          (`self.AutoSpawn Item In SLOT` "/Game/VR_Inventorys/Items/BP_CrowBar.BP_CrowBar_C"))
        (:`NewEnumerator10`
          (`self.AutoSpawn Item In SLOT` "/Game/VR_Inventorys/Items/BP_FireAxe.BP_FireAxe_C"))
        (:`NewEnumerator11`
          (`self.AutoSpawn Item In SLOT` "/Game/VR_Inventorys/Items/BP_FireAxe_Composit.BP_FireAxe_Composit_C"))
        (:`NewEnumerator12`
          (`self.AutoSpawn Item In SLOT` "/Game/VR_Inventorys/Items/BP_DoubleHead_Axe.BP_DoubleHead_Axe_C"))
        (:`NewEnumerator14`
          (`self.AutoSpawn Item In SLOT` "/Game/VR_Inventorys/Items/BP_BaseBallBat_Wood.BP_BaseBallBat_Wood_C"))
        (:`NewEnumerator16`
          (`self.AutoSpawn Item In SLOT` "/Game/VR_Inventorys/Items/BP_BaseBallBat_Alloy.BP_BaseBallBat_Alloy_C"))
        (:`NewEnumerator15`
          (`self.AutoSpawn Item In SLOT` "/Game/VR_Inventorys/Items/BP_Hatchete.BP_Hatchete_C"))
        (:`NewEnumerator17`
          (`self.AutoSpawn Item In SLOT` "/Game/VR_Inventorys/Items/BP_VR_FlashLight_1.BP_VR_FlashLight_1_C"))
        (:`NewEnumerator18`
          (`self.AutoSpawn Item In SLOT` "/Game/VR_Inventorys/Items/BP_VR_FlashLight_2.BP_VR_FlashLight_2_C"))))
    (:`then_7`
      ;[1 1 1] Set Haptic effects from slot Config, If nonthing is set Use a Default Haptic effect to avoid the accessed None error!
      (`/Engine/EditorBlueprintResources/StandardMacros.IsValid` `Store Item Haptic`
        (:`Is Valid`
          (set `self.Slot Configuration Slotted Haptic Effect` `Store Item Haptic`))
        (:`Is Not Valid`
          (set `self.Slot Configuration Slotted Haptic Effect` "/Game/VR_Inventorys/VRTemplate/Haptics/HolsterSelectionHover.HolsterSelectionHover"))))
    (:`then_8`
      (`/Engine/EditorBlueprintResources/StandardMacros.IsValid` `Slot Detect Haptic`
        (:`Is Valid`
          (set `self.Slot Configuration Interaction Haptic Effect` `Slot Detect Haptic`))
        (:`Is Not Valid`
          (set `self.Slot Configuration Interaction Haptic Effect` "/Game/VR_Inventorys/VRTemplate/Haptics/SelectionHover.SelectionHover"))))))

(fn `Update Slot Colour`
  (params (`Correct Colour` :type "LinearColor Structure") (`Wrong Colour` :type "LinearColor Structure"))
  (bind (_slot_configuration_dontshowouterring _slot_configuration_dontshowslottext _slot_configuration_dontshowemptysloticon _slot_configuration_sizescalingoninteraction _slot_configuration_opacityscalingoninteraction _slot_configuration_rotationoninteraction _slot_configuration_slotcolor _slot_configuration_outerringcolor _slot_configuration_slottype) (break `/Game/VR_Inventorys/Blueprints/Struct_Slot_Config` (`self.Slot configuration`)))
  (bind _slot_dynamic_mat (`self.Slot Dynamic Mat`))
  ;[0 0 0] Check slot type and change color for player Clue!
  (if (`|EnumEquality` (`/Game/VR_Inventorys/Blueprints/BP_VRM_GrabComponent.SlotType` (`self.Detected Item`)) _slot_configuration_slottype)
    (`MaterialInstanceDynamic.SetVectorParameterValue` _slot_dynamic_mat "Color" `Correct Colour`)
    (else
      (`MaterialInstanceDynamic.SetVectorParameterValue` _slot_dynamic_mat "Color" `Wrong Colour`)))
  (return))

(fn `Update Slot Opacity`
  (params (Value :type "Float (single-precision)"))
  (bind (_slot_configuration_dontshowouterring _slot_configuration_dontshowslottext _slot_configuration_dontshowemptysloticon _slot_configuration_sizescalingoninteraction _slot_configuration_opacityscalingoninteraction) (break `/Game/VR_Inventorys/Blueprints/Struct_Slot_Config` (`self.Slot configuration`)))
  (if _slot_configuration_opacityscalingoninteraction
    (`MaterialInstanceDynamic.SetScalarParameterValue` (`self.Slot Dynamic Mat`) "MinOpacity" Value)))

(fn `UserConstructionScript`)