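; VR inventory "AUTO" slot that routes an item to a free slot of the same type in its parent inventory.
; AutoStore scans the attach parent's child slots and sends AutoStoreMessage to the first unused match, then breaks the loop.
; Any occupied match found before that briefly turns the label to a red "Full".
; Overlap by an actor with a grab component drives a timeline that rescales the slot mesh.
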(event `self.ReceiveTick`
  (params (DeltaSeconds :type "Float (single-precision)"))
  (`KismetSystemLibrary.Delay` 1.0))

(event `/Game/VR_Inventorys/Blueprints/BPI_InventorySlot_Interface.Auto Store`
  (params (`Slot type` :type "/Game/VR_Inventorys/Blueprints/Enum_Inventory_slotType Enum" :default "NewEnumerator0") (ACTOR :type "Actor Object Reference") (`Skeletal Mesh` :type "SkeletalMeshComponent Object Reference") (`Static mesh` :type "StaticMeshComponent Object Reference") (`Primitive Component` :type "PrimitiveComponent Object Reference") (`Pawn Held Component Ref ` :type "/Game/VR_Inventorys/Blueprints/BP_VRM_GrabComponent Object Reference") (`Motion Controller` :type "MotionControllerComponent Object Reference"))
  (bind _returnvalue (`self.GetAttachParentActor`))
  (bind _name_ (`self.name `))
  (bind _name__2 (`self.name `))
  ;[0.0716 0.5955 0 0.573] Get all slots of Inventory parent actor,  excluding  This Auto slot
  (`/Engine/EditorBlueprintResources/StandardMacros.IsValid` _returnvalue
    (:`Is Valid`
      (for _array_element (`self.GetAllChildActors` _returnvalue false) :!label _label
        (bind _asbp_inventory_slot_base (cast `/Game/VR_Inventorys/Slots/BASE_SLOT/BP_Inventory_Slot_BASE` _array_element :!pure true))
        (`/Engine/EditorBlueprintResources/StandardMacros.IsValid` _asbp_inventory_slot_base
          (:`Is Valid`
            (bind _slot_in_use (`/Game/VR_Inventorys/Slots/BASE_SLOT/BP_Inventory_Slot_BASE.Slot in Use` _asbp_inventory_slot_base))
            (bind (_slot_configuration_dontshowouterring _slot_configuration_dontshowslottext _slot_configuration_dontshowemptysloticon _slot_configuration_sizescalingoninteraction _slot_configuration_opacityscalingoninteraction _slot_configuration_rotationoninteraction _slot_configuration_slotcolor _slot_configuration_outerringcolor _slot_configuration_slottype) (break `/Game/VR_Inventorys/Blueprints/Struct_Slot_Config` (`/Game/VR_Inventorys/Slots/BASE_SLOT/BP_Inventory_Slot_BASE.Slot configuration` _asbp_inventory_slot_base)))
            (bind _returnvalue_2 (`|EnumEquality` _slot_configuration_slottype `Slot type`))
            (if (and (not _slot_in_use) _returnvalue_2)
              (message `/Game/VR_Inventorys/Blueprints/BPI_InventorySlot_Interface.Auto Store` _array_element "NewEnumerator0" ACTOR null null `Primitive Component` null `Motion Controller`)
              (`self.Stop Loop`)
              (elif (and _returnvalue_2 _slot_in_use)
                ;[1 1 1] Change slot text to TO DISPLAY FULL MESSAGE for a second  when trying to auto slot a item type that there are no empty solts left for
                (`TextRenderComponent.K2_SetText` _name__2 "Full")
                (`TextRenderComponent.SetTextRenderColor` _name__2 (`KismetMathLibrary.Conv_LinearColorToColor` (`KismetMathLibrary.MakeColor` 1.0)))
                (`KismetSystemLibrary.Delay` 1.0)
                (`TextRenderComponent.K2_SetText` _name_ "AUTO")
                (`TextRenderComponent.SetTextRenderColor` _name_ (`KismetMathLibrary.Conv_LinearColorToColor` (`KismetMathLibrary.MakeColor` 1.0 1.0 1.0)))))))))))

(event `Stop Loop`
  ;[0.0716 0.5955 0 0.573] Get all slots of Inventory parent actor,  excluding  This Auto slot
  (goto _label :!via `Break`))

(event `self.Trigger Detect Box.OnComponentBeginOverlap`
  (params (OverlappedComponent :type "PrimitiveComponent Object Reference") (OtherActor :type "Actor Object Reference") (OtherComp :type "PrimitiveComponent Object Reference") (OtherBodyIndex :type Integer) (bFromSweep :type Boolean) (SweepResult :type "HitResult Structure (by ref)"))
  ;[0.9812 1 0 0] Potential Slot Interaction when Hand Hover over Occupied slot
  (if (`KismetSystemLibrary.IsValid` (`self.GetComponentByClass` OtherActor "/Game/VR_Inventorys/Blueprints/BP_VRM_GrabComponent.BP_VRM_GrabComponent_C"))
    (bind (_direction _lerp) (`Timeline|Timeline_0` :!label _label_2)
      (:`Update`
        ;;[1 1 1] Scale Up Slot Mesh, On Hover (relative to its parent actor
        (`SceneComponent.SetRelativeScale3D` (`self.style mesh`) (`KismetMathLibrary.VLerp` (1.0 1.0 10.0) (1.3 1.3 1.0) _lerp))))))

(event `self.Trigger Detect Box.OnComponentEndOverlap`
  (params (OverlappedComponent :type "PrimitiveComponent Object Reference") (OtherActor :type "Actor Object Reference") (OtherComp :type "PrimitiveComponent Object Reference") (OtherBodyIndex :type Integer))
  ;[0.9812 1 0 0] Potential Slot Interaction when Hand Hover over Occupied slot
  (if (`KismetSystemLibrary.IsValid` (`self.GetComponentByClass` OtherActor "/Game/VR_Inventorys/Blueprints/BP_VRM_GrabComponent.BP_VRM_GrabComponent_C"))
    (goto _label_2 :!via `Reverse`)))

(fn `UserConstructionScript`)